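; BP_Monster is a placeholder monster Blueprint that exercises Gameplay Ability System activation and shows its health for debugging.
; On BeginPlay, a looping timer calls TestAbility, which tries to activate the first ability returned by its ability system component.
; Tick prints the current health to the screen every frame.
; An activate-by-class call using the CharacterAbilities array is left unconnected and never runs.
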(event `self.ReceiveBeginPlay`
  (`KismetSystemLibrary.K2_SetTimer` null "TestAbility" 1.0 true))

(event `TestAbility`
  (bind _outabilityhandles (`AbilitySystemComponent.GetAllAbilities` (`self.HardRefAbilitySystemComponent`)))
  (`AbilitySystemComponent.TryActivateAbility` (`self.HardRefAbilitySystemComponent`) (`|GetArrayItem` _outabilityhandles) true))

(event `self.ReceiveTick`
  (params (DeltaSeconds :type "Float (single-precision)"))
  (`KismetSystemLibrary.PrintString` (`KismetStringLibrary.Conv_DoubleToString` (`self.GetHealth`)) true true (struct :`G` 0.66 :`B` 1.0 :`A` 1.0) 0.0))

(fn `UserConstructionScript`)