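; A placeholder test player character for exercising Gameplay Ability System abilities, attributes and death.
; On BeginPlay it adds an Enhanced Input mapping, grants each character ability bound to the same attack action, and prints attribute changes from the PlayerState's ability system.
; A debug D key applies a set-by-caller damage effect to itself and calls Die when no longer alive; the death event prints a message.
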(event Custom|OnCharacterDied_Event
  (params (Character :type Character%20Base%20Object%20Reference))
  (Development|PrintString "Died"))

(event EventBeginPlay
  (bind _enhancedinputasc (Variables|Default|GetEnhancedInputASC))
  (EventDispatchers|AssignOnCharacterDied (delegate Custom|OnCharacterDied_Event))
  (bind _asplayer_controller (Utilities|Casting|CastToPlayerController (Pawn|GetController)))
  (Utilities|IsValid (PlayerController|LocalPlayerSubsystems|GetEnhancedInputLocalPlayerSubsystem _asplayer_controller)
    (:Is%20Valid
      (Input|AddMappingContext (PlayerController|LocalPlayerSubsystems|GetEnhancedInputLocalPlayerSubsystem _asplayer_controller) "/Game/Inputs/IMC_WheelDefault.IMC_WheelDefault" 0 "(bIgnoreAllPressedKeysUntilRelease=True,bForceImmediately=False)")
      (for _array_element (Variables|Default|GetCharacterAbilities)
        (bind _returnvalue (GameplayAbilities|GiveAbility _enhancedinputasc _array_element 0 -1))
        (Class|EnhancedInputASC|SetInputBinding _enhancedinputasc "/Game/Inputs/InputActions/IA_Attack.IA_Attack" _returnvalue)
        (bind _ascharacter_player_state (Utilities|Casting|CastToCharacterPlayerState (Variables|Default|GetPlayerState)))
        (bind (_asynctaskproxy _attribute _newvalue _oldvalue) (|ListenforAttributeChange (Ability|GetAbilitySystemComponent _ascharacter_player_state) "(AttributeName=\"Health\",Attribute=/Script/Curseel.AttributeSetBase:Health,AttributeOwner=/Script/CoreUObject.Class'\"/Script/Curseel.AttributeSetBase\"')")
          (:OnAttributeChanged
            (Development|PrintString (Utilities|String|Append (.attributename _attribute) " New : " (Utilities|String|ToString(Float) _newvalue) " Old : " (Utilities|String|ToString(Float) _oldvalue)) true true "(R=0.000000,G=0.660000,B=1.000000,A=1.000000)" 1.0)))))))

(event Input|KeyboardEvents|DebugKeyD
  (params (Key :type Key%20Structure) (ActionValue :type Input%20Action%20Value%20Structure))
  (:Pressed
    (bind _ascharacter_player_state (Utilities|Casting|CastToCharacterPlayerState (Variables|Default|GetPlayerState)))
    ;[1 1 1] Attribute Attack + Magnitude = BaseDamage
    (bind _returnvalue (Ability|GameplayEffect|AssignTagSetbyCallerMagnitude (GameplayEffects|MakeOutgoingSpec (Ability|GetAbilitySystemComponent _ascharacter_player_state) "/Game/Placeholder/GE_Damage.GE_Damage_C" 0.0 (GameplayEffects|MakeEffectContext (Ability|GetAbilitySystemComponent _ascharacter_player_state))) "(TagName=\"Data.Damage\")" (Variables|Default|GetMagnitude)))
    (GameplayEffects|ApplyGameplayEffectSpecToSelf (Ability|GetAbilitySystemComponent _ascharacter_player_state) _returnvalue)
    (if (not (Class|CharacterBase|IsAlive))
      (Class|CharacterBase|Die))))

(fn ConstructionScript)