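; Dialogue manager that plays data table dialogues one at a time, with character-specific lines when sigils activate, finish or have a boost chosen.
; Each row is sent to the pawn and HUD with 2D audio, held for its duration, then advanced.
; With a level sequence, it pauses the sequence after each line until ContinueDialogue is called, auto-continuing only on the last.
; Finishing via ContinueDialogue restores wheel input from cutscene input.
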(event `OnSigilActivation`
  (params (Sigil :type "/Game/Dungeon/Sigil/BP_Sigil Object Reference"))
  ;[1 1 1] Sigils dialogues
  (`self.TryToStartDialogue` (select `int` (`WheelPawn.CurrentCharacterIndex` (`self.Wheel`)) :`0` "/Game/Dialogues/Barks/DT_StartFight_Benelu.DT_StartFight_Benelu" :`1` "/Game/Dialogues/Barks/DT_StartFight_Kyana.DT_StartFight_Kyana" :`2` "/Game/Dialogues/Barks/DT_StartFight_Tolg.DT_StartFight_Tolg" :!type "DataTable Object Reference")))

(event `OnSigilFinish`
  (params (Sigil :type "/Game/Dungeon/Sigil/BP_Sigil Object Reference"))
  ;[1 1 1] Sigils dialogues
  (`self.TryToStartDialogue` (select `int` (`WheelPawn.CurrentCharacterIndex` (`self.Wheel`)) :`0` "/Game/Dialogues/Barks/DT_EndFight_Benelu.DT_EndFight_Benelu" :`1` "/Game/Dialogues/Barks/DT_EndFight_Kyana.DT_EndFight_Kyana" :`2` "/Game/Dialogues/Barks/DT_EndFight_Tolg.DT_EndFight_Tolg" :!type "DataTable Object Reference")))

(event `OnBoostChosen_Event`
  ;[1 1 1] Sigils dialogues
  (`self.TryToStartDialogue` (select `int` (`WheelPawn.CurrentCharacterIndex` (`self.Wheel`)) :`0` "/Game/Dialogues/Barks/DT_Boost_Benelu.DT_Boost_Benelu" :`1` "/Game/Dialogues/Barks/DT_Boost_Kyana.DT_Boost_Kyana" :`2` "/Game/Dialogues/Barks/DT_Boost_Tolg.DT_Boost_Tolg" :!type "DataTable Object Reference")))

(event `self.ReceiveBeginPlay`
  (message `/Game/GameModes/BPI_CurseelGM.SetDialogueManager` (`GameplayStatics.GetGameMode`) self)
  (bind _asbp_wheel (cast `/Game/Wheel/BP_Wheel` (`GameplayStatics.GetPlayerPawn` 0)))
  (set `self.Wheel` _asbp_wheel)
  ;[1 1 1] Sigils dialogues
  (bind _outactors (`GameplayStatics.GetAllActorsOfClass` "/Game/Dungeon/Sigil/BP_Sigil.BP_Sigil_C"))
  (for _array_element _outactors
    (`|ExecutionSequence`
      (:`then_0`
        (add `/Game/Dungeon/Sigil/BP_Sigil.OnActivated` _array_element (delegate `OnSigilActivation`)))
      (:`then_1`
        (add `/Game/Dungeon/Sigil/BP_Sigil.OnFinish` _array_element (delegate `OnSigilFinish`)))
      (:`then_2`
        (add `/Game/Dungeon/Sigil/BP_Sigil.OnBoostChosen` _array_element (delegate `OnBoostChosen_Event`))))))

(event `StopCurrentDialogue`
  (`/Engine/EditorBlueprintResources/StandardMacros.IsValid` (`self.CurrentDialogue`)
    (:`Is Valid`
      (`self.StopDialogue`))))

(event `StartDialogue`
  (params (Index :type Integer))
  (set `self.CurIndex` Index)
  (bind _outrownames (`DataTableFunctionLibrary.GetDataTableRowNames` (`self.CurrentDialogue`)))
  (if (`self.HasDialogue` (`self.CurIndex`))
    (bind _returnvalue (`|GetDataTableRow` (`self.CurrentDialogue`) (`|GetArrayItem` _outrownames (`self.CurIndex`)))
      (:`then`
        (set `self.bIsShowing` true)
        (message `/Game/Dialogues/BPI_Dialogue.ShowDialogue` (`GameplayStatics.GetPlayerPawn` 0) _returnvalue)
        (message `/Game/Dialogues/BPI_Dialogue.ShowDialogue` (`PlayerController.GetHUD` (`GameplayStatics.GetPlayerController` 0)) _returnvalue)
        (bind (_speakingcharacter _content _duration _dialogueaudio) (break `/Game/Dialogues/S_Dialogue` _returnvalue))
        (`self.PlayAudio` _dialogueaudio)
        (`KismetSystemLibrary.RetriggerableDelay` _duration)
        (`self.ToggleSequence` false)
        (set `self.bIsShowing` false)
        (`/Engine/EditorBlueprintResources/StandardMacros.IsValid` (`self.CurrentSequence`)
          (:`Is Valid`
            ;[1 1 1] AutoFinish on last dialogue
            (if (not (`self.HasNextDialogue` (`self.CurIndex`)))
              (`self.ContinueDialogue`)))
          (:`Is Not Valid`
            (`self.ContinueDialogue`))))
      (:`RowNotFound`
        (`self.StopDialogue` :!label _label)))
    (else
      (goto _label))))

(event `ContinueDialogue`
  (bind _curindex (`self.CurIndex`))
  (if (not (`self.bIsShowing`))
    (`self.ToggleSequence` true)
    (set `self.bIsHiding` true)
    (message `/Game/Dialogues/BPI_Dialogue.HideDialogue` (`GameplayStatics.GetPlayerPawn` 0))
    (message `/Game/Dialogues/BPI_Dialogue.HideDialogue` (`PlayerController.GetHUD` (`GameplayStatics.GetPlayerController` 0)))
    (`KismetSystemLibrary.RetriggerableDelay` 0.5)
    (set `self.bIsHiding` false)
    (if (`self.HasNextDialogue` _curindex)
      (`self.StartDialogue` (+ _curindex 1))
      (else
        (`self.StopDialogue`)
        (`CurseelBlueprintFunctionLibrary.RemoveCutsceneInput` (pcsubsystem `EnhancedInputLocalPlayerSubsystem` (`GameplayStatics.GetPlayerController` 0)) "/Game/Inputs/IMC_Cutscene.IMC_Cutscene" "/Game/Inputs/IMC_Wheel.IMC_Wheel")))))

(fn `HasDialogue`
  (params (CurrentIndex :type Integer))
  (returns (ReturnValue :type Boolean))
  (bind _outrownames (`DataTableFunctionLibrary.GetDataTableRowNames` (`self.CurrentDialogue`)))
  (return (<= CurrentIndex (`KismetArrayLibrary.Array_LastIndex` _outrownames))))

(fn `HasNextDialogue`
  (params (CurrentIndex :type Integer))
  (returns (ReturnValue :type Boolean))
  (return (`self.HasDialogue` (+ CurrentIndex 1))))

(fn `InDialogue`
  (returns (ReturnValue :type Boolean))
  (return (`KismetSystemLibrary.IsValid` (`self.CurrentDialogue`))))

(fn `PlayAudio`
  (params (Audio :type "SoundWave Object Reference"))
  (`/Engine/EditorBlueprintResources/StandardMacros.IsValid` Audio
    (:`Is Valid`
      (`GameplayStatics.PlaySound2D` Audio 1.0 1.0 0.0 null null))))

(fn `StopDialogue`
  (set `self.CurrentDialogue` null)
  (set `self.CurIndex` -2)
  (`self.OnDialogueFinished`)
  (return))

(fn `ToggleSequence`
  (params (Play :type Boolean))
  (bind _currentsequence (`self.CurrentSequence`))
  (`/Engine/EditorBlueprintResources/StandardMacros.IsValid` _currentsequence
    (:`Is Valid`
      (if Play
        (`MovieSceneSequencePlayer.Play` _currentsequence)
        (else
          (`MovieSceneSequencePlayer.Pause` _currentsequence))))))

(fn `TryToStartDialogue`
  (params (NewDialogue :type "DataTable Object Reference") (LevelSequencePlayer :type "LevelSequencePlayer Object Reference"))
  (returns (Suceeded :type Boolean))
  (`/Engine/EditorBlueprintResources/StandardMacros.IsValid` NewDialogue
    (:`Is Valid`
      (`/Engine/EditorBlueprintResources/StandardMacros.IsValid` (`self.CurrentDialogue`)
        (:`Is Valid`
          _)
        (:`Is Not Valid`
          (set `self.CurrentDialogue` NewDialogue)
          (set `self.CurrentSequence` LevelSequencePlayer)
          (`self.StartDialogue` 0)
          (return true))))
    (:`Is Not Valid`
      _))
  (return false))

(fn `UserConstructionScript`)