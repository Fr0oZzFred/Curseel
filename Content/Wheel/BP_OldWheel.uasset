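; Player pawn that drives a "wheel" of three child-actor characters (DD, healer, tank) as one unit, with pooled health and averaged move speed.
; Turning cycles the current character, re-laying out the formation around it; attacks fire on all three, while the GAS skill uses only the current one.
; Enhanced Input handles movement, cooldown-gated turn and dash, and stick aiming, with mouse aiming polled on Tick.
; Damage updates the life gauge, low-health vignette and game over.
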(event `UpdateShield`
  (params (Value :type "Float (double-precision)"))
  (set `self.Shield` (`KismetMathLibrary.FClamp` (+ (`self.Shield`) Value) 0.0 (`self.MaxShield`))))

(event `AddCombo`
  (params (ComboPassCount :type Integer))
  (bind _result (`/Engine/EditorBlueprintResources/StandardMacros.IncrementInt` (`self.ComboPassCount`))
    (:`  `
      (if (> _result 2)
        (bind _output_get (set `self.CurComboScore` (+ (stale _output_get) ComboPassCount)))
        (set `self.ComboPassCount` 0)
        (`self.OnCombo` (stale _output_get_2))
        (bind _output_get_2 (set `self.CurComboScore` 0))
        (else
          (bind _output_get_3 (set `self.CurComboScore` (+ (stale _output_get_3) ComboPassCount))))))))

(event `CustomEvent`
  (params (Character :type "CharacterBase Object Reference"))
  (`self.UpdateMS`))

(event `OnCharacterHealthChanged_Event`
  (params (Character :type "CharacterBase Object Reference") (NewHealth :type "Float (single-precision)") (OldHealth :type "Float (single-precision)"))
  (bind _vignetteanim (`self.VignetteAnim`))
  (`self.OnHealthChanged`)
  (bind _output_get (set `self.Health` (- (stale _output_get) (- OldHealth NewHealth))))
  (`self.UpdateCenter` 0.0)
  (bind _returnvalue (/ _output_get (`self.MaxHealth`)))
  (if (< _returnvalue 0.0)
    (`self.OnDied` null)
    (elif (< _returnvalue 0.4)
      (if (not (`TimelineComponent.IsPlaying` (`self.VignetteAnim`)))
        (bind (_direction _radius) (`Timeline|VignetteAnim` :!via `PlayFromStart`)
          (:`Update`
            (`KismetMaterialLibrary.SetScalarParameterValue` (`self.MPC_Vignette`) "RadiusNormalized" _radius))))
      (elif (`TimelineComponent.IsPlaying` _vignetteanim)
        (`TimelineComponent.Stop` _vignetteanim)
        (`TimelineComponent.SetNewTime` (`self.VignetteAnim`) 0.0)))))

(event `self.ReceiveTick`
  (params (DeltaSeconds :type "Float (single-precision)"))
  (bind _returnvalue (`GameplayStatics.GetPlayerController` 0))
  (set `self.DT` DeltaSeconds)
  (`AISense_Hearing.ReportNoiseEvent` (`self.K2_GetActorLocation`) 1.0 self)
  (bind _returnvalue_2 (`WidgetLayoutLibrary.GetMousePositionOnViewport`))
  (if (!= _returnvalue_2 (`self.OldMousePosition`) :`ErrorTolerance` 5.0)
    (set `self.OldMousePosition` _returnvalue_2)
    (if (`self.UsingMouse`)
      (`WidgetBlueprintLibrary.SetInputMode_GameAndUIEx` _returnvalue null)
      (else
        (set `self.UsingMouse` true)
        (`WidgetBlueprintLibrary.SetInputMode_GameAndUIEx` _returnvalue null)
        (set `PlayerController.bShowMouseCursor` true _returnvalue)))
    (bind (_x _y) (`KismetMathLibrary.BreakVector2D` (`KismetMathLibrary.Normal2D` (- (`WidgetLayoutLibrary.ProjectWorldLocationToWidgetPosition` _returnvalue (`SceneComponent.K2_GetComponentLocation` (`self.WheelCenter`))) _returnvalue_2))))
    (`SceneComponent.K2_SetRelativeRotation` (`self.WheelOrientation`) (`KismetMathLibrary.MakeRotator` 0.0 0.0 (* (`KismetMathLibrary.DegAtan2` _x _y) -1.0)) false false)
    (else
      (set `self.OldMousePosition` _returnvalue_2))))

(event `self.ReceiveBeginPlay`
  (bind _returnvalue (pcsubsystem `EnhancedInputLocalPlayerSubsystem` (cast `PlayerController` (`self.GetController`) :!pure true)))
  (`/Engine/EditorBlueprintResources/StandardMacros.IsValid` _returnvalue
    (:`Is Valid`
      (`EnhancedInputSubsystemInterface.AddMappingContext` _returnvalue "/Game/Inputs/IMC_Wheel.IMC_Wheel" 0 (struct))
      (`EnhancedInputSubsystemInterface.AddMappingContext` _returnvalue "/Game/Inputs/IMC_SystemInGame.IMC_SystemInGame" 10 (struct)))
    (:`Is Not Valid`
      (`KismetSystemLibrary.PrintString` "Input Local not valid")))
  (`self.InitCharacters`)
  (`self.SetFormationWheelFront`)
  (set `self.TwinStick` true)
  (`self.UpdateColor`)
  (`|ExecutionSequence`
    (:`then_0`
      (for _array_element (`self.Characters`)
        (add `CharacterBase.OnCharacterHealthChanged` _array_element (delegate `OnCharacterHealthChanged_Event`))
        (`self.UpdateCenter` 0.0)
        (add `CharacterBase.OnCharacterMoveSpeedChanged` _array_element (delegate `CustomEvent`))))
    (:`then_1`
      (`self.UpdateCurCharacter`) ; Hardcoded for UI
      (bind _outactors (`GameplayStatics.GetAllActorsOfClass` "/Game/Monsters/BP_MonstersPackArea.BP_MonstersPackArea_C"))
      (if (== (`KismetArrayLibrary.Array_Length` _outactors) 1)
        (set `self.MonstersPack` (`|GetArrayItem` _outactors))
        (else
          (`KismetSystemLibrary.PrintString` "Monsters Pack missing or more than 1 instance"))))
    (:`then_2`
      (add `self.OnWheelTurn` (delegate `UpdateCenter`)))))

(event `OnDied`
  (params (Character :type "CharacterBase Object Reference"))
  (if (not (`self.Invincible`))
    (`/Game/GameModes/InGame/HUD_InGame.ActivateGameOverMenu` (`self.HUD_InGame`))
    (`self.Die`)))

(event `UpdateCenter` :!signature `self.OnWheelTurn`
  (params (TurnCD :type "Float (double-precision)"))
  (`MeshComponent.SetScalarParameterValueOnMaterials` (`self.LifeGauge`) "Life" (/ (`self.Health`) (`self.MaxHealth`))))

(event `TryToTurnWheel`
  (params (Clockwise :type Boolean))
  (if (not (`self.TurnOnCD`))
    (if (`self.TwinStick`)
      (`self.TurnWheelFront` Clockwise)
      (else
        (`self.TurnWheel` Clockwise)))
    (`self.UpdateColor`)
    (set `self.TurnOnCD` true)
    (`KismetSystemLibrary.Delay` (`self.TurnWheelCD`))
    (set `self.TurnOnCD` false)))

(event `TryToDash`
  (if (not (`self.DashOnCD`))
    (`self.Dash`)
    (set `self.DashOnCD` true)
    (`TimelineComponent.SetPlayRate` (`self.Timeline`) (/ 1.0 (`self.DashCD`)))
    (bind (_direction _progression) (`Timeline|Timeline` :!via `PlayFromStart`)
      (:`Update`
        (`MeshComponent.SetScalarParameterValueOnMaterials` (`self.DashJauge`) "Progression" _progression))
      (:`Finished`
        (set `self.DashOnCD` false)))))

(event `EnhancedInput|/Game/Inputs/InputActions/IA_Move`
  (params (ActionValue :type "Vector2D Structure") (ElapsedSeconds :type "Float (double-precision)") (TriggeredSeconds :type "Float (double-precision)") (InputAction :type "InputAction Object Reference" :default "/Game/Inputs/InputActions/IA_Move.IA_Move"))
  (bind (_returnvalue_roll _returnvalue_pitch _returnvalue_yaw) (`KismetMathLibrary.BreakRotator` (`self.GetControlRotation`)))
  (bind (_returnvalue_roll_2 _returnvalue_pitch_2 _returnvalue_yaw_2) (`KismetMathLibrary.BreakRotator` (`self.GetControlRotation`)))
  (bind _floatingpawnmovement (`self.FloatingPawnMovement`))
  ;[0.2 0.2 0.2 1 100] Inputs
  ;;[1 1 1] Movement
  (:`Triggered`
    (`|ExecutionSequence`
      (:`then_0`
        (`PawnMovementComponent.AddInputVector` _floatingpawnmovement (* (`KismetMathLibrary.GetRightVector` (`KismetMathLibrary.MakeRotator` _returnvalue_roll_2 0.0 _returnvalue_yaw_2)) ActionValue_X) false))
      (:`then_1`
        (`PawnMovementComponent.AddInputVector` _floatingpawnmovement (* (`KismetMathLibrary.GetForwardVector` (`KismetMathLibrary.MakeRotator` 0.0 0.0 _returnvalue_yaw)) ActionValue_Y) false)))))

(event `EnhancedInput|/Game/Inputs/InputActions/IA_Turn`
  (params (ActionValue :type "Float (double-precision)") (ElapsedSeconds :type "Float (double-precision)") (TriggeredSeconds :type "Float (double-precision)") (InputAction :type "InputAction Object Reference" :default "/Game/Inputs/InputActions/IA_Turn.IA_Turn"))
  ;[0.2 0.2 0.2 1 100] Inputs
  ;;[1 1 1] Turns
  (:`Triggered`
    (`self.TryToTurnWheel` (> ActionValue 0.0))))

(event `EnhancedInput|/Game/Inputs/InputActions/IA_Dash`
  (params (ActionValue :type Boolean) (ElapsedSeconds :type "Float (double-precision)") (TriggeredSeconds :type "Float (double-precision)") (InputAction :type "InputAction Object Reference" :default "/Game/Inputs/InputActions/IA_Dash.IA_Dash"))
  ;[0.2 0.2 0.2 1 100] Inputs
  ;;[1 1 1] Dash
  (:`Triggered`
    (`self.TrytoDash`)))

(event `EnhancedInput|/Game/Inputs/InputActions/IA_Attack`
  (params (ActionValue :type Boolean) (ElapsedSeconds :type "Float (double-precision)") (TriggeredSeconds :type "Float (double-precision)") (InputAction :type "InputAction Object Reference" :default "/Game/Inputs/InputActions/IA_Attack.IA_Attack"))
  ;[0.2 0.2 0.2 1 100] Inputs
  ;;[1 1 1] Attack
  (:`Triggered`
    (for _array_element (`self.Characters`)
      (`/Game/MainCharacters/OldDesign/BP_WheelCharacter.Attack` _array_element))))

(event `EnhancedInput|/Game/Inputs/InputActions/IA_Orientation`
  (params (ActionValue :type "Vector2D Structure") (ElapsedSeconds :type "Float (double-precision)") (TriggeredSeconds :type "Float (double-precision)") (InputAction :type "InputAction Object Reference" :default "/Game/Inputs/InputActions/IA_Orientation.IA_Orientation"))
  (bind (_x _y) (`KismetMathLibrary.BreakVector2D` ActionValue))
  (bind (_x_2 _y_2) (`KismetMathLibrary.BreakVector2D` ActionValue))
  (bind _returnvalue (`GameplayStatics.GetPlayerController` 0))
  (bind _wheelorientation (`self.WheelOrientation`))
  (bind (_relativerotation_roll _relativerotation_pitch _relativerotation_yaw) (`KismetMathLibrary.BreakRotator` (`SceneComponent.RelativeRotation` _wheelorientation)))
  ;[0.2 0.2 0.2 1 100] Inputs
  ;;[1 1 1] Orientation Input
  (:`Triggered`
    (if (`self.TwinStick`)
      (set `self.UsingMouse` false)
      (`WidgetBlueprintLibrary.SetInputMode_GameOnly` _returnvalue)
      (set `PlayerController.bShowMouseCursor` false _returnvalue)
      (`SceneComponent.K2_SetRelativeRotation` (`self.WheelOrientation`) (`KismetMathLibrary.MakeRotator` 0.0 0.0 (* (`KismetMathLibrary.DegAtan2` _x_2 _y_2) -1.0)) false false)
      (else
        (`SceneComponent.K2_SetRelativeRotation` _wheelorientation (`KismetMathLibrary.MakeRotator` 0.0 0.0 (`KismetMathLibrary.Lerp` _relativerotation_yaw (/ (* (`KismetMathLibrary.DegAtan2` _x (`KismetMathLibrary.FClamp` _y)) -1.0) 3.0) (* (`self.DT`) (`self.AlphaRot`)))) false false)))))

(event `EnhancedInput|/Game/Inputs/InputActions/IA_Skill`
  (params (ActionValue :type Boolean) (ElapsedSeconds :type "Float (double-precision)") (TriggeredSeconds :type "Float (double-precision)") (InputAction :type "InputAction Object Reference" :default "/Game/Inputs/InputActions/IA_Skill.IA_Skill"))
  ;[0.2 0.2 0.2 1 100] Inputs
  ;;[1 1 1] Skill
  (:`Triggered`
    (if (`self.UseSkills`)
      (bind _currentcharacter (`self.GetCurCharacter`))
      (bind _output (`|GetArrayItem` (`CharacterBase.Abilities` _currentcharacter) 1))
      (bind _returnvalue (`AbilitySystemComponent.TryActivateAbilityByClass` (`WheelCharacter.HardRefAbilitySystemComponent` _currentcharacter) _output true))
      (if _returnvalue
        _
        (elif (`KismetSystemLibrary.IsValidClass` _output)
          (`KismetSystemLibrary.PrintString` "SKILL NOT READY")
          (else
            (`KismetSystemLibrary.PrintString` "SKILL NOT SET")))))))

(event `EnhancedInput|/Game/Inputs/InputActions/IA_Pause`
  (params (ActionValue :type Boolean) (ElapsedSeconds :type "Float (double-precision)") (TriggeredSeconds :type "Float (double-precision)") (InputAction :type "InputAction Object Reference" :default "/Game/Inputs/InputActions/IA_Pause.IA_Pause"))
  (bind _hud_ingame (`self.HUD_InGame`))
  ;[0.2 0.2 0.2 1 100] Inputs
  ;;[1 1 1] Pause
  (:`Triggered`
    (`/Engine/EditorBlueprintResources/StandardMacros.IsValid` _hud_ingame
      (:`Is Valid`
        (`/Game/GameModes/InGame/HUD_InGame.OpenPauseMenu` _hud_ingame))
      (:`Is Not Valid`
        (`KismetSystemLibrary.PrintString` "HUD In Game not valid")))))

(event `EnhancedInput|/Game/Inputs/InputActions/IA_Interact`
  (params (ActionValue :type Boolean) (ElapsedSeconds :type "Float (double-precision)") (TriggeredSeconds :type "Float (double-precision)") (InputAction :type "InputAction Object Reference" :default "/Game/Inputs/InputActions/IA_Interact.IA_Interact"))
  ;[0.2 0.2 0.2 1 100] Inputs
  ;;[1 1 1] Interact
  (:`Triggered`
    (`self.OnInteract`)))

(event `EnhancedInput|/Game/Inputs/InputActions/IA_ChangeFormation`
  (params (ActionValue :type Boolean) (ElapsedSeconds :type "Float (double-precision)") (TriggeredSeconds :type "Float (double-precision)") (InputAction :type "InputAction Object Reference" :default "/Game/Inputs/InputActions/IA_ChangeFormation.IA_ChangeFormation"))
  ;[0.2 0.2 0.2 1 100] Inputs
)

(fn `Dash`
  (bind _output_get (set `MovementComponent.Velocity` (* (`KismetMathLibrary.Normal` (stale _output_get)) (`self.DashForce`)) (`self.FloatingPawnMovement`)))
  (`self.OnDash` (`self.DashCD`)))

(fn `Die`
  (bind _returnvalue (pcsubsystem `EnhancedInputLocalPlayerSubsystem` (cast `PlayerController` (`self.GetController`) :!pure true)))
  (set `FloatingPawnMovement.MaxSpeed` 0.0 (`self.FloatingPawnMovement`))
  (`|ExecutionSequence`
    (:`then_0`
      (`/Engine/EditorBlueprintResources/StandardMacros.IsValid` _returnvalue
        (:`Is Valid`
          (`EnhancedInputSubsystemInterface.RemoveMappingContext` _returnvalue "/Game/Inputs/IMC_Wheel.IMC_Wheel" (struct)))
        (:`Is Not Valid`
          (`KismetSystemLibrary.PrintString` "Input Local not valid"))))
    (:`then_1`
      (return))))

(fn `GetCurCharacter`
  (returns (CurrentCharacter :type "/Game/MainCharacters/OldDesign/BP_WheelCharacter Object Reference"))
  (return (cast `/Game/MainCharacters/OldDesign/BP_WheelCharacter` (`ChildActorComponent.ChildActor` (`|GetArrayItem` (`|MakeArray` (`self.BP_DDCharacter`) (`self.BP_HealerCharacter`) (`self.BP_TankCharacter`)) (`self.CurCharacterIndex`))) :!pure true)))

(fn `GetLeftCharacter`
  (returns (LeftCharacter :type "/Game/MainCharacters/OldDesign/BP_WheelCharacter Object Reference"))
  (return (cast `/Game/MainCharacters/OldDesign/BP_WheelCharacter` (`ChildActorComponent.ChildActor` (`|GetArrayItem` (`|MakeArray` (`self.BP_DDCharacter`) (`self.BP_HealerCharacter`) (`self.BP_TankCharacter`)) (mod (+ (`self.CurCharacterIndex`) -1 3) 3))) :!pure true)))

(fn `GetRightCharacter`
  (returns (RightCharacter :type "/Game/MainCharacters/OldDesign/BP_WheelCharacter Object Reference"))
  (return (cast `/Game/MainCharacters/OldDesign/BP_WheelCharacter` (`ChildActorComponent.ChildActor` (`|GetArrayItem` (`|MakeArray` (`self.BP_DDCharacter`) (`self.BP_HealerCharacter`) (`self.BP_TankCharacter`)) (mod (+ (`self.CurCharacterIndex`) 1 3) 3))) :!pure true)))

(fn `InitCharacters`
  (locals (TotalMoveSpeed :type "Float (double-precision)") (CharactersLength :type Integer :default 0))
  (bind _array (`|MakeArray` (`self.BP_DDCharacter`) (`self.BP_HealerCharacter`) (`self.BP_TankCharacter`)))
  (set `local.CharactersLength` (`KismetArrayLibrary.Array_Length` _array))
  (for _array_element _array
    (bind _asbp_wheel_character (cast `/Game/MainCharacters/OldDesign/BP_WheelCharacter` (`ChildActorComponent.ChildActor` _array_element) :!pure true))
    (`KismetArrayLibrary.Array_Add` (`self.Characters`) _asbp_wheel_character)
    (bind _output_get (set `local.TotalMoveSpeed` (+ (stale _output_get) (`CharacterMovementComponent.MaxWalkSpeed` (`Character.CharacterMovement` _asbp_wheel_character)))))
    (`self.SetOwner` _asbp_wheel_character self)
    (bind _output_get_2 (set `self.MaxHealth` (+ (stale _output_get_2) (`CharacterBase.GetMaxHealth` _asbp_wheel_character)))))
  ;[1 1 1] Average Speed
  (bind _output_get_3 (set `FloatingPawnMovement.MaxSpeed` (/ (`local.TotalMoveSpeed`) (`local.CharactersLength`)) (`self.FloatingPawnMovement`)))
  (set `self.MoveSpeed` _output_get_3)
  (set `self.Health` (`self.MaxHealth`)))

(fn `PredicLocation`
  (bind _returnvalue (`self.GetTransform`))
  (bind (_outradius _outhalfheight) (`CapsuleComponent.GetScaledCapsuleSize` (`self.Capsule`)))
  (bind _returnvalue_2 (`KismetMathLibrary.TransformLocation` _returnvalue (* (`MovementComponent.Velocity` (`self.FloatingPawnMovement`)) (`self.PredicTime`))))
  (bind (_outhit _returnvalue_3) (`KismetSystemLibrary.LineTraceSingleForObjects` :`Start` (.location _returnvalue) :`End` _returnvalue_2 :`ObjectTypes` (`|MakeArray` "ObjectTypeQuery1" :!type "EObjectTypeQuery Enum") :`DrawDebugType` "ForOneFrame"))
  (bind _output_get (set `self.PredicLoc` (select `bool` _returnvalue_3 :`false` _returnvalue_2 :`true` (`.Location` (`GameplayStatics.BreakHitResult` _outhit)))))
  (if (`self.DebugPredicLocation`)
    (`KismetSystemLibrary.DrawDebugCapsule` _output_get _outhalfheight _outradius (struct) (struct :`R` 1.0 :`G` 1.0 :`B` 1.0 :`A` 1.0) 0.0 10.0)))

(fn `SetFormationHugeWheel`
  (bind _array (`|MakeArray` (`self.CharacterFront`) (`self.CharacterRight`) (`self.CharacterLeft`)))
  (for (_array_element _array_index) _array
    (`SceneComponent.ResetRelativeTransform` _array_element)
    (bind _returnvalue (* (`KismetMathLibrary.GetTAU`) (/ (`KismetMathLibrary.Conv_IntToDouble` _array_index) (`KismetMathLibrary.Conv_IntToDouble` (`KismetArrayLibrary.Array_Length` _array)))))
    (`SceneComponent.K2_SetRelativeLocationAndRotation` :`self` _array_element :`NewLocation` (* (`KismetMathLibrary.MakeVector` (`KismetMathLibrary.Cos` _returnvalue) (`KismetMathLibrary.Sin` _returnvalue)) (`self.HugeWheelRadius`)))
    (`SceneComponent.K2_SetRelativeRotation` _array_element (.rotation (`KismetAnimationLibrary.K2_LookAt` (`SceneComponent.GetRelativeTransform` _array_element) (`KismetMathLibrary.MakeVector` 0.0) (1.0 0.0 0.0))) false false)
    (`CapsuleComponent.SetCapsuleSize` (`self.Capsule`) 550.0 750.0 true)))

(fn `SetFormationWheel`
  (bind _array (`|MakeArray` (`self.CharacterFront`) (`self.CharacterRight`) (`self.CharacterLeft`)))
  (for (_array_element _array_index) _array
    (`SceneComponent.ResetRelativeTransform` _array_element)
    (bind _returnvalue (* (`KismetMathLibrary.GetTAU`) (/ (`KismetMathLibrary.Conv_IntToDouble` _array_index) (`KismetMathLibrary.Conv_IntToDouble` (`KismetArrayLibrary.Array_Length` _array)))))
    (bind _returnvalue_2 (`KismetMathLibrary.MakeVector` (`KismetMathLibrary.Cos` _returnvalue) (`KismetMathLibrary.Sin` _returnvalue)))
    (`SceneComponent.K2_SetRelativeLocationAndRotation` _array_element (* _returnvalue_2 (`self.WheelRadius`)) (.rotation (`KismetAnimationLibrary.K2_LookAt` (`SceneComponent.GetRelativeTransform` _array_element) _returnvalue_2 (1.0 0.0 0.0))) false false)
    (`CapsuleComponent.SetCapsuleSize` (`self.Capsule`) 140.0 280.0 true)))

(fn `SetFormationWheelFront`
  (bind _returnvalue (select `int` (`self.CurCharacterIndex`) :`0` (`|MakeArray` (`self.CharacterFront`) (`self.CharacterRight`) (`self.CharacterLeft`)) :`1` (`|MakeArray` (`self.CharacterRight`) (`self.CharacterLeft`) (`self.CharacterFront`)) :`2` (`|MakeArray` (`self.CharacterLeft`) (`self.CharacterFront`) (`self.CharacterRight`))))
  (for (_array_element _array_index) _returnvalue
    (`SceneComponent.ResetRelativeTransform` _array_element)
    (bind _returnvalue_2 (* (select `int` _array_index :`0` 4.0 :`1` 4.0 :`2` (* 4.0 -1.0)) (/ (`KismetMathLibrary.Conv_IntToDouble` (`KismetMathLibrary.Clamp` _array_index 0 1)) (`KismetMathLibrary.Conv_IntToDouble` (`KismetArrayLibrary.Array_Length` _returnvalue)))))
    (bind _returnvalue_3 (`KismetMathLibrary.MakeVector` (`KismetMathLibrary.Cos` _returnvalue_2) (`KismetMathLibrary.Sin` _returnvalue_2)))
    (`SceneComponent.K2_SetRelativeLocationAndRotation` _array_element (* _returnvalue_3 (`self.WheelRadius`)) (.rotation (`KismetAnimationLibrary.K2_LookAt` (`SceneComponent.GetRelativeTransform` _array_element) _returnvalue_3 (1.0 0.0 0.0))) false false)
    (`CapsuleComponent.SetCapsuleSize` (`self.Capsule`) 140.0 280.0 true)))

(fn `TurnWheel`
  (params (Clockwise :type Boolean))
  (locals (NewFront :type "SceneComponent Object Reference"))
  (bind _returnvalue (/ 360.0 3.0))
  ;[1 1 1] Update Cur Index
  (set `self.CurCharacterIndex` (mod (+ (`self.CurCharacterIndex`) (select `bool` Clockwise :`false` 1 :`true` -1) 3) 3))
  (`SceneComponent.K2_AddRelativeRotation` (`self.WheelCenter`) (`KismetMathLibrary.MakeRotator` 0.0 0.0 (select `bool` (`local.Clockwise`) :`false` (* _returnvalue -1.0) :`true` _returnvalue :!type "Float (single-precision)")) false false)
  (`self.UpdateCurCharacter`)
  (`self.OnWheelTurn` (`self.TurnWheelCD`)))

(fn `TurnWheelFront`
  (params (Clockwise :type Boolean))
  (locals (NewFront :type "SceneComponent Object Reference"))
  ;[1 1 1] Update Cur Index
  (set `self.CurCharacterIndex` (mod (+ (`self.CurCharacterIndex`) (select `bool` Clockwise :`false` 1 :`true` -1) 3) 3))
  (`self.SetFormationWheelFront`)
  (`self.UpdateCurCharacter`)
  (`self.OnWheelTurn` (`self.TurnWheelCD`)))

(fn `UpdateCurCharacter`
  (bind _currentcharacter (`self.GetCurCharacter`))
  (set `self.CurrentCharacter` _currentcharacter)
  (return))

(fn `UpdateMS`
  (locals (TotalSpeed :type "Float (single-precision)" :default 0.0))
  (for _array_element (`self.Characters`)
    (bind _output_get (set `local.TotalSpeed` (+ (stale _output_get) (`CharacterBase.GetMoveSpeed` _array_element)))))
  (set `FloatingPawnMovement.MaxSpeed` (/ (`local.TotalSpeed`) 3.0) (`self.FloatingPawnMovement`)))

(fn `UserConstructionScript`
  (`self.SetFormationWheelFront`))