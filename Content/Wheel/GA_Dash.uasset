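; GA_Dash is the Gameplay Ability that makes BP_Wheel dash.
; On commit it applies GE_GenericDashCooldown with an attribute-driven duration, replaces the FloatingMovement velocity with CalcDir's result, and ends immediately.
; CalcDir picks aim or last-move direction from a GI_Curseel setting, with a world +X fallback, and DashPower scales by attributes.
; The Ability.ExplosiveDash tag also enables the wheel's explosive dash.
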(event `self.K2_ActivateAbility`
  (bind _returnvalue (`self.GetAvatarActorFromActorInfo`))
  (bind _wheel (`self.Wheel`))
  (bind _wheel_2 (`self.Wheel`))
  (bind _returnvalue_2 (`AbilitySystemBlueprintLibrary.GetAbilitySystemComponent` (`self.GetAvatarActorFromActorInfo`)))
  (bind (_lastmovevalue_x _lastmovevalue_y) (`KismetMathLibrary.BreakVector2D` (`WheelPawn.LastMoveValue` _wheel)))
  (bind _floatingmovement (`WheelPawn.FloatingMovement` (`self.Wheel`)))
  (bind _returnvalue_3 (select `bool` (`/Game/Blueprints/GI_Curseel.DashToDirection` (cast `/Game/Blueprints/GI_Curseel` (`GameplayStatics.GetGameInstance`) :!pure true)) :`false` (`KismetMathLibrary.Normal` (`KismetMathLibrary.MakeVector` _lastmovevalue_y _lastmovevalue_x)) :`true` (`WheelPawn.AimDirection` _wheel)))
  (bind _returnvalue_4 (`self.K2_CommitAbility`))
  (if _returnvalue_4
    (bind _asbp_wheel (cast `/Game/Wheel/BP_Wheel` _returnvalue))
    (set `self.Wheel` _asbp_wheel)
    (bind _returnvalue_5 (`AbilitySystemBlueprintLibrary.SetDuration` (`AbilitySystemComponent.MakeOutgoingSpec` _returnvalue_2 "/Game/Wheel/GE_GenericDashCooldown.GE_GenericDashCooldown_C" 0.0 (`AbilitySystemComponent.MakeEffectContext` _returnvalue_2)) (`.ReturnValue` (`AbilitySystemBlueprintLibrary.GetFloatAttribute` _returnvalue (struct :`AttributeName` "DashCooldown" :`Attribute` "/Script/Curseel.AttributeSetBase:DashCooldown" :`AttributeOwner` "/Script/CoreUObject.Class'\"/Script/Curseel.AttributeSetBase\"'")))))
    (`AbilitySystemComponent.BP_ApplyGameplayEffectSpecToSelf` _returnvalue_2 _returnvalue_5)
    (`|ExecutionSequence`
      (:`then_0`
        ;[1 1 1] Dash
        (set `self.NewVelocity` (* (select `bool` (== _returnvalue_3 (0.0 0.0 0.0)) :`false` _returnvalue_3 :`true` (1.0 0.0 0.0)) (`.ReturnValue` (`AbilitySystemBlueprintLibrary.GetFloatAttribute` (`self.GetAvatarActorFromActorInfo`) (struct :`AttributeName` "DashPower" :`Attribute` "/Script/Curseel.AttributeSetBase:DashPower" :`AttributeOwner` "/Script/CoreUObject.Class'\"/Script/Curseel.AttributeSetBase\"'")))))
        (`MovementComponent.StopMovementImmediately` _floatingmovement)
        (set `MovementComponent.Velocity` (`self.NewVelocity`) _floatingmovement))
      (:`then_1`
        ;[1 1 1] Check Explosive Dash
        (if (`GameplayTagAssetInterface.HasMatchingGameplayTag` (`AbilitySystemBlueprintLibrary.GetAbilitySystemComponent` _wheel_2) (struct :`TagName` "Ability.ExplosiveDash"))
          (`/Game/Wheel/BP_Wheel.EnableExplosiveDash` _wheel_2)))
      (:`then_2`
        (`self.K2_EndAbility`)))))