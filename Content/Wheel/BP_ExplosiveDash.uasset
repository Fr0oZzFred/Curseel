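; Child actor of BP_Wheel that knocks monsters aside while the wheel dashes.
; CheckForCollision enables Tick, which polls capsule overlaps while the Ability.Dash tag is present and velocity exceeds move speed, then disables itself and clears the hit list.
; Each monster is hit once, with an impulse along the swapped X/Y velocity, signed by a dot product with its wheel-relative position.
; Dash damage is only a placeholder print.
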(event `self.ReceiveBeginPlay`
  (bind _asbp_wheel (cast `/Game/Wheel/BP_Wheel` (`self.GetParentActor`)))
  (set `self.Wheel` _asbp_wheel))

(event `self.ReceiveTick`
  (params (DeltaSeconds :type "Float (single-precision)"))
  (if (`self.IsDashing`)
    (`self.CheckMonsterCollision`)
    (else
      (`self.DisableExplosiveDash`))))

(event `CheckForCollision`
  (`self.SetActorTickEnabled` true))

(fn `ApplyEffects`
  (params (MonsterCharacter :type "/Game/Monsters/BP_MonsterCharacter Object Reference"))
  (bind _knockbackpower (`self.KnockbackPower`))
  (bind _charactermovement (`Character.CharacterMovement` (`local.MonsterCharacter`)))
  (bind (_x _y) (`KismetMathLibrary.BreakVector3f` (`MovementComponent.Velocity` (`WheelPawn.FloatingMovement` (`self.Wheel`)))))
  (bind _returnvalue (`KismetMathLibrary.Normal` (`KismetMathLibrary.MakeVector` _y _x)))
  (bind _returnvalue_2 (select `bool` (> (`KismetMathLibrary.Dot_VectorVector` _returnvalue (`KismetMathLibrary.Normal` (`KismetMathLibrary.InverseTransformLocation` (`self.GetTransform` (`self.Wheel`)) (`self.K2_GetActorLocation` (`local.MonsterCharacter`))))) 0.0) :`false` (* _knockbackpower -1.0) :`true` _knockbackpower))
  (`|ExecutionSequence`
    (:`then_0`
      ;[1 1 1] Knockback
      (`MovementComponent.StopMovementImmediately` _charactermovement)
      (`CharacterMovementComponent.AddImpulse` _charactermovement (* _returnvalue (`KismetMathLibrary.MakeVector` _returnvalue_2 _returnvalue_2)) true))
    (:`then_1`
      (`KismetSystemLibrary.PrintString` "Implement Dash Damage"))))

(fn `CheckMonsterCollision`
  (bind _touchedactor (`self.TouchedActor`))
  (for _array_element (`PrimitiveComponent.GetOverlappingActors` (`self.Capsule`) "/Game/Monsters/BP_MonsterCharacter.BP_MonsterCharacter_C")
    (bind _asbp_monster_character (cast `/Game/Monsters/BP_MonsterCharacter` _array_element))
    (if (== (`KismetArrayLibrary.Array_Find` _touchedactor _array_element) -1)
      (`KismetArrayLibrary.Array_Add` _touchedactor _array_element)
      (`self.ApplyEffects` _asbp_monster_character)))
  (return))

(fn `DisableExplosiveDash`
  (`self.SetActorTickEnabled` false)
  (`KismetArrayLibrary.Array_Clear` (`self.TouchedActor`)))

(fn `IsDashing`
  (returns (ReturnValue :type Boolean))
  (bind _wheel (`self.Wheel`))
  (return (and (`GameplayTagAssetInterface.HasMatchingGameplayTag` (`AbilitySystemBlueprintLibrary.GetAbilitySystemComponent` _wheel) (struct :`TagName` "Ability.Dash")) (> (`KismetMathLibrary.VSize` (`MovementComponent.Velocity` (`WheelPawn.FloatingMovement` _wheel))) (`PawnBase.GetMoveSpeed` _wheel)))))

(fn `UserConstructionScript`
  (`CapsuleComponent.SetCapsuleSize` (`self.Capsule`) (`self.Radius`) (`self.HalfHeight`) false))