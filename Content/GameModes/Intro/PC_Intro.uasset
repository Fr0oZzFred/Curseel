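; Player controller for the intro that handles cutscene input for skipping and advancing dialogue.
; On BeginPlay it adds the cutscene Enhanced Input mapping context and focuses the game.
; Skip input fires the OnTrySkipIntro dispatcher, while a separate SkipIntro event fires OnSkipIntro.
; Continue input casts the game mode to GM_Intro and tells its DialogueManager to continue the dialogue.
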(event `self.ReceiveBeginPlay`
  (bind _returnvalue (pcsubsystem `EnhancedInputLocalPlayerSubsystem` self))
  (`/Engine/EditorBlueprintResources/StandardMacros.IsValid` _returnvalue
    (:`Is Valid`
      (`EnhancedInputSubsystemInterface.AddMappingContext` _returnvalue "/Game/Inputs/IMC_Cutscene.IMC_Cutscene" 11 (struct))
      (`CurseelBlueprintFunctionLibrary.FocusGame` self))))

(event `EnhancedInput|/Game/Inputs/InputActions/IA_SkipCutscene`
  (params (ActionValue :type Boolean) (ElapsedSeconds :type "Float (double-precision)") (TriggeredSeconds :type "Float (double-precision)") (InputAction :type "InputAction Object Reference" :default "/Game/Inputs/InputActions/IA_SkipCutscene.IA_SkipCutscene"))
  (:`Triggered`
    (`self.OnTrySkipIntro`)))

(event `EnhancedInput|/Game/Inputs/InputActions/IA_ContinueCutscene`
  (params (ActionValue :type Boolean) (ElapsedSeconds :type "Float (double-precision)") (TriggeredSeconds :type "Float (double-precision)") (InputAction :type "InputAction Object Reference" :default "/Game/Inputs/InputActions/IA_ContinueCutscene.IA_ContinueCutscene"))
  (:`Triggered`
    (`/Game/Dialogues/BP_DialogueManager.ContinueDialogue` (`/Game/GameModes/Intro/GM_Intro.Dialogue Manager` (cast `/Game/GameModes/Intro/GM_Intro` (`GameplayStatics.GetGameMode`) :!pure true)))))

(event `SkipIntro`
  (`self.OnSkipIntro`))

(fn `UserConstructionScript`)