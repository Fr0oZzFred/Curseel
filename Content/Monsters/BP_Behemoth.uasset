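; BP_Behemoth is a monster Blueprint that extends its parent's behavior to drive a big-monster animation Blueprint.
; On BeginPlay it runs the parent logic, then casts the mesh's anim instance to ABP_BigMonster and caches it.
; Each Tick runs the parent logic, then pushes the result of GetSpeed into the anim instance's Speed variable.
; The construction script only calls the parent's.
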(event `self.ReceiveBeginPlay`
  (`parent.ReceiveBeginPlay`)
  (bind _asabp_big_monster (cast `/Game/Monsters/BigMonster/ABP_BigMonster` (`SkeletalMeshComponent.GetAnimInstance` (`self.Mesh`))))
  (set `self.ABP_BigMonster` _asabp_big_monster))

(event `self.ReceiveTick`
  (params (DeltaSeconds :type "Float (single-precision)"))
  (`parent.ReceiveTick` DeltaSeconds)
  (set `/Game/Monsters/BigMonster/ABP_BigMonster.Speed` (`self.GetSpeed`) (`self.ABP_BigMonster`)))

(fn `UserConstructionScript`
  (`parent.UserConstructionScript`))