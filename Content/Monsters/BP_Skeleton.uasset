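; BP_Skeleton is a skeleton monster Blueprint that drives its animation Blueprint with its movement speed.
; On BeginPlay it casts the mesh's anim instance to ABP_Skeleton and caches the reference.
; Each Tick it pushes the result of GetSpeed into that instance's Speed variable.
; BeginPlay, Tick and the construction script all call their parent versions, and the construction script adds nothing of its own.
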(event `self.ReceiveBeginPlay`
  (`parent.ReceiveBeginPlay`)
  (bind _asabp_skeleton (cast `/Game/Monsters/Skeleton/ABP_Skeleton` (`SkeletalMeshComponent.GetAnimInstance` (`self.Mesh`))))
  (set `self.ABP_Skeleton` _asabp_skeleton))

(event `self.ReceiveTick`
  (params (DeltaSeconds :type "Float (single-precision)"))
  (`parent.ReceiveTick` DeltaSeconds)
  (set `/Game/Monsters/Skeleton/ABP_Skeleton.Speed` (`self.GetSpeed`) (`self.ABP_Skeleton`)))

(fn `UserConstructionScript`
  (`parent.UserConstructionScript`))