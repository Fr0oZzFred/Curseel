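; Monster pack area actor that keeps itself centered between the player and a capped group of monster AI controllers.
; Each tick, construction or Refresh moves it to the averaged X/Y of the monsters' pawns and player 0.
; AddMonster registers controllers up to MaxMonsters and assigns them the pack navigation query filter.
; RemoveMonster unregisters them without restoring the previous filter.
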(event `self.ReceiveTick`
  (params (DeltaSeconds :type "Float (single-precision)"))
  (`self.MoveActorToCenter` :!label _label))

(event `Refresh`
  (goto _label))

(fn `AddMonster`
  (params (MonsterController :type "AIController Object Reference (by ref)"))
  (bind _monstercontroller (`local.MonsterController`))
  (bind _monsterspackactors (`self.MonstersPackActors`))
  (if (`KismetArrayLibrary.Array_Contains` _monsterspackactors MonsterController)
    _
    (elif (>= (`KismetArrayLibrary.Array_Length` _monsterspackactors) (`self.MaxMonsters`))
      (`KismetSystemLibrary.PrintString` "Blocked")
      (else
        (`KismetArrayLibrary.Array_Add` (`self.MonstersPackActors`) _monstercontroller)
        (set `AIController.DefaultNavigationFilterClass` "/Game/Monsters/BP_QueryFilter_MonstersPack.BP_QueryFilter_MonstersPack_C" _monstercontroller)
        (`KismetSystemLibrary.PrintString` "Added")))))

(fn `MoveActorToCenter`
  (bind (_returnvalue_x _returnvalue_y) (`KismetMathLibrary.BreakVector` (/ (`self.Centroid`) (`KismetMathLibrary.Conv_IntToDouble` (+ (`KismetArrayLibrary.Array_Length` (`self.MonstersPackActors`)) 1)))))
  (set `self.Centroid` (0.0 0.0 0.0))
  (for _array_element (`self.MonstersPackActors`)
    (`/Engine/EditorBlueprintResources/StandardMacros.IsValid` _array_element
      (:`Is Valid`
        (bind _output_get (set `self.Centroid` (+ (stale _output_get) (`self.K2_GetActorLocation` (`Controller.K2_GetPawn` _array_element))))))))
  (bind _output_get_2 (set `self.Centroid` (+ (stale _output_get_2) (`self.K2_GetActorLocation` (`GameplayStatics.GetPlayerPawn` 0)))))
  (`self.K2_SetActorLocation` (`KismetMathLibrary.MakeVector` _returnvalue_x _returnvalue_y)))

(fn `RemoveMonster`
  (params (MonsterController :type "AIController Object Reference (by ref)"))
  (if (`KismetArrayLibrary.Array_Contains` (`self.MonstersPackActors`) MonsterController)
    (`KismetArrayLibrary.Array_RemoveItem` (`self.MonstersPackActors`) (`local.MonsterController`))
    (`KismetSystemLibrary.PrintString` "Removed")))

(fn `UserConstructionScript`
  (`self.MoveActorToCenter`))