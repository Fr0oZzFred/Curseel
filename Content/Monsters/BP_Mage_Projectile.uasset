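; BP_Mage_Projectile is a mage monster's projectile that flies toward the player and damages wheel characters.
; On BeginPlay it aims once at the player pawn's position, with zero vertical velocity.
; Sphere overlap destroys it on static meshes; on a WheelCharacter it applies GE_GenericDamage to that character via SetByCaller, reduced by the player's Shield, then drains that shield and destroys itself.
; The impact sound is unconnected.
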(event `self.ReceiveBeginPlay`
  (bind _projectilemovement (`self.ProjectileMovement`))
  (bind _initialspeed (`ProjectileMovementComponent.InitialSpeed` _projectilemovement))
  (set `MovementComponent.Velocity` (* (`KismetMathLibrary.Normal` (- (`self.K2_GetActorLocation` (`GameplayStatics.GetPlayerPawn` 0)) (`self.K2_GetActorLocation`))) (`KismetMathLibrary.MakeVector` _initialspeed _initialspeed)) _projectilemovement))

(event `self.Sphere.OnComponentBeginOverlap`
  (params (OverlappedComponent :type "PrimitiveComponent Object Reference") (OtherActor :type "Actor Object Reference") (OtherComp :type "PrimitiveComponent Object Reference") (OtherBodyIndex :type Integer) (bFromSweep :type Boolean) (SweepResult :type "HitResult Structure (by ref)"))
  (bind _asbp_wheel (cast `/Game/Wheel/BP_OldWheel` (`GameplayStatics.GetPlayerPawn` 0) :!pure true))
  (cast `StaticMeshActor` OtherActor
    (:`then`
      (`self.K2_DestroyActor`))
    (:`CastFailed`
      (bind _aswheel_character (cast `WheelCharacter` OtherActor))
      (bind _returnvalue (`AbilitySystemBlueprintLibrary.GetAbilitySystemComponent` _aswheel_character))
      (bind _returnvalue_2 (`AbilitySystemBlueprintLibrary.AssignTagSetByCallerMagnitude` (`AbilitySystemComponent.MakeOutgoingSpec` _returnvalue "/Game/Blueprints/GE_GenericDamage.GE_GenericDamage_C" 0.0 (`AbilitySystemComponent.MakeEffectContext` _returnvalue)) (struct :`TagName` "Data.Damage") (- (`self.Damage`) (`/Game/Wheel/BP_OldWheel.Shield` _asbp_wheel))))
      (`AbilitySystemComponent.BP_ApplyGameplayEffectSpecToSelf` _returnvalue _returnvalue_2)
      (`/Game/Wheel/BP_OldWheel.UpdateShield` _asbp_wheel (* (`self.Damage`) -1.0))
      (`self.K2_DestroyActor`))))

(fn `UserConstructionScript`)