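; BP_Wolf is a monster Blueprint that drives its mesh animation from the creature's movement speed.
; On BeginPlay, after the parent logic, it casts the mesh's anim instance to ABP_Skeleton, despite the wolf name, and caches it.
; Each Tick then copies GetSpeed into that anim Blueprint's Speed variable, and the construction script only calls the parent.
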(event `self.ReceiveBeginPlay`
  (`parent.ReceiveBeginPlay`)
  (bind _asabp_skeleton (cast `/Game/Monsters/Skeleton/ABP_Skeleton` (`SkeletalMeshComponent.GetAnimInstance` (`self.Mesh`))))
  (set `self.ABP_Skeleton` _asabp_skeleton))

(event `self.ReceiveTick`
  (params (DeltaSeconds :type "Float (single-precision)"))
  (`parent.ReceiveTick` DeltaSeconds)
  (set `/Game/Monsters/Skeleton/ABP_Skeleton.Speed` (`self.GetSpeed`) (`self.ABP_Skeleton`)))

(fn `UserConstructionScript`
  (`parent.UserConstructionScript`))