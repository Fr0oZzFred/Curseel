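; Monster character that chases and attacks the player's wheel pawn, with a 3D life bar widget linked to its owner.
; ChasePlayer sets blackboard keys for its AI, while Attack activates the first Gameplay Ability and turns the monster toward the player on success.
; On death it waits a tick to avoid an attribute-set error, leaves the game mode's monster pack, plays a random sound and destroys itself.
; The construction script can add a debug sphere showing attack range.
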(event `ChasePlayer`
  (bind _returnvalue (`AIBlueprintHelperLibrary.GetBlackboard` null))
  (`BlackboardComponent.SetValueAsObject` _returnvalue "Player" (`GameplayStatics.GetPlayerPawn` 0))
  (`BlackboardComponent.SetValueAsBool` _returnvalue "ChasingPlayer" true))

(event `self.ReceiveBeginPlay`
  (add `self.OnCharacterDied` (delegate `OnCharacterDied_Event`))
  (`|ExecutionSequence`
    (:`then_0`
      (set `self.PlayerWheel` (cast `/Game/Wheel/BP_Wheel` (`GameplayStatics.GetPlayerPawn` 0) :!pure true)))
    (:`then_1`
      (set `/Game/UI/W_LifeBar3D.OwnerCharacter` self (cast `/Game/UI/W_LifeBar3D` (`WidgetComponent.GetWidget` (`self.W_LifeBar`)) :!pure true)))))

(event `OnCharacterDied_Event` :!signature `self.OnCharacterDied`
  (params (Character :type "CharacterBase Object Reference"))
  (`KismetSystemLibrary.DelayUntilNextTick`) ; Avoid error at PostGameplayEffectExecute in AttributeSetBase
  (`/Game/Monsters/BP_MonstersPackArea.RemoveMonster` (`/Game/GameModes/InGame/GM_InGame.MonstersPack` (cast `/Game/GameModes/InGame/GM_InGame` (`GameplayStatics.GetGameMode`) :!pure true)) (`AIBlueprintHelperLibrary.GetAIController` self))
  (`GameplayStatics.PlaySound2D` (`KismetArrayLibrary.Array_Random` (`|MakeArray` "/Game/Placeholder/Audio/michelbaradari-monsters/deathb.deathb" "/Game/Placeholder/Audio/michelbaradari-monsters/deathe.deathe" "/Game/Placeholder/Audio/michelbaradari-monsters/deathr.deathr" "/Game/Placeholder/Audio/michelbaradari-monsters/deaths.deaths" :!type "SoundBase Object Reference")) 1.0 1.0 0.0 null null)
  (`self.K2_DestroyActor`))

(event `Attack`
  (bind _returnvalue (`AbilitySystemComponent.TryActivateAbilityByClass` (`self.HardRefAbilitySystemComponent`) (`|GetArrayItem` (`self.Abilities`)) true))
  (if _returnvalue
    (`self.K2_SetActorRotation` (`KismetMathLibrary.MakeRotator` 0.0 0.0 (.yaw (.rotation (`KismetAnimationLibrary.K2_LookAt` (`self.GetTransform`) (`self.K2_GetActorLocation` (`self.PlayerWheel`)) (1.0 0.0 0.0))))))))

(fn `UserConstructionScript`
  (bind _debugsphere (`self.DebugSphere`))
  (bind _debugsphere_2 (`self.DebugSphere`))
  (if (`self.DebugAttackRange`)
    (`/Engine/EditorBlueprintResources/StandardMacros.IsValid` (`self.DebugSphere`)
      (:`Is Not Valid`
        (bind _returnvalue (`AddComponent|NODE_AddSphereComponent-0` :`bManualAttachment` true))
        (set `self.DebugSphere` _returnvalue)
        (`|ExecutionSequence`
          (:`then_0`
            (`PrimitiveComponent.SetCollisionEnabled` _debugsphere "NoCollision")
            (`SphereComponent.SetSphereRadius` _debugsphere (`self.AttackRange`) false))
          (:`then_1`
            (`SceneComponent.SetHiddenInGame` _debugsphere_2 false false)
            (`SceneComponent.K2_AttachToComponent` _debugsphere_2 (`self.Mesh`) "None" "SnapToTarget" "SnapToTarget" "KeepWorld" true)))))
    (else
      (`/Engine/EditorBlueprintResources/StandardMacros.IsValid` (`self.DebugSphere`)
        (:`Is Valid`
          (`ActorComponent.K2_DestroyComponent` (`self.DebugSphere`)))))))