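; Area-of-effect ability for the Behemoth monster, adding a character reaction line when its effect is applied.
; ApplyEffect runs the parent logic, then asks the GM_InGame DialogueManager to try starting a big-damage dialogue.
; The dialogue table is selected from the player BP_Wheel's current character index: Benelu, Kyana or Tolg.
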(event `self.ApplyEffect`
  (params (Actor :type "Actor Object Reference") (TouchedASC :type "AbilitySystemComponent Object Reference"))
  (`parent.ApplyEffect` Actor TouchedASC)
  (bind _asbp_wheel (cast `/Game/Wheel/BP_Wheel` (`GameplayStatics.GetPlayerPawn` 0)))
  (bind _asgm_in_game (cast `/Game/GameModes/InGame/GM_InGame` (`GameplayStatics.GetGameMode`)))
  (`/Game/Dialogues/BP_DialogueManager.TryToStartDialogue` (`/Game/GameModes/InGame/GM_InGame.DialogueManager` _asgm_in_game) (select `int` (`WheelPawn.CurrentCharacterIndex` _asbp_wheel) :`0` "/Game/Dialogues/Barks/DT_BigDamage_Benelu.DT_BigDamage_Benelu" :`1` "/Game/Dialogues/Barks/DT_BigDamage_Kyana.DT_BigDamage_Kyana" :`2` "/Game/Dialogues/Barks/DT_BigDamage_Tolg.DT_BigDamage_Tolg" :!type "DataTable Object Reference") null))

(fn `UserConstructionScript`
  (`parent.UserConstructionScript`))