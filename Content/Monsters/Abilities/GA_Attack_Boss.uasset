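; GA_Attack_Boss is the boss monster's attack gameplay ability, spawning a randomly chosen attack AOE on activation.
; It binds to the avatar's destruction and, for a CharacterBase avatar, its stun event, then commits the ability before spawning from AttackAOEs.
; The avatar-destroyed, stun and AOE-destroyed events all defer to parent class handlers.
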(event `self.K2_ActivateAbility`
  (bind _returnvalue (`self.GetAvatarActorFromActorInfo`))
  (add `Actor.OnDestroyed` _returnvalue (delegate `self.OnAvatarActorDestroyed`))
  (bind _ascharacter_base (cast `CharacterBase` _returnvalue)
    (:`then`
      (add `CharacterBase.OnCharacterStunned` _ascharacter_base (delegate `self.OnCharacterStunned_Event`)))
    (:`CastFailed`
      _))
  (bind _returnvalue_2 (`self.K2_CommitAbility`))
  (if _returnvalue_2
    (bind _spawnedaoe (`self.SpawnAOE` (`KismetArrayLibrary.Array_Random` (`self.AttackAOEs`))))
    (add `Actor.OnDestroyed` _spawnedaoe (delegate `self.OnAOE_Destroyed`))))

(event `self.OnAOE_Destroyed`
  (params (DestroyedActor :type "Actor Object Reference"))
  (`parent.OnAOE_Destroyed` DestroyedActor))

(event `self.OnAvatarActorDestroyed`
  (params (DestroyedActor :type "Actor Object Reference"))
  (`parent.OnAvatarActorDestroyed` DestroyedActor))

(event `self.OnCharacterStunned_Event`
  (params (Character :type "CharacterBase Object Reference") (Stunned :type Boolean))
  (`parent.OnCharacterStunned_Event` Character Stunned))