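; Mage monster projectile that flies toward the player and deals Gameplay Ability System damage on overlap.
; On BeginPlay it aims once at player 0's location with vertical velocity zeroed, so it does not home, and caches the owner's ability system component.
; Sphere overlap destroys it on static mesh actors, ignores the owner, and otherwise applies GE_GenericDamage with tag-set magnitude before destroying itself.
; The impact sound is unwired.
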(event `self.ReceiveBeginPlay`
  (bind _projectilemovement (`self.ProjectileMovement`))
  (bind _initialspeed (`ProjectileMovementComponent.InitialSpeed` _projectilemovement))
  (set `MovementComponent.Velocity` (* (`KismetMathLibrary.Normal` (- (`self.K2_GetActorLocation` (`GameplayStatics.GetPlayerPawn` 0)) (`self.K2_GetActorLocation`))) (`KismetMathLibrary.MakeVector` _initialspeed _initialspeed)) _projectilemovement)
  (bind _returnvalue (`CurseelBlueprintFunctionLibrary.GetCurseelASC` (`self.GetOwner`)))
  (set `self.OwnerASC` _returnvalue))

(event `self.Sphere.OnComponentBeginOverlap`
  (params (OverlappedComponent :type "PrimitiveComponent Object Reference") (OtherActor :type "Actor Object Reference") (OtherComp :type "PrimitiveComponent Object Reference") (OtherBodyIndex :type Integer) (bFromSweep :type Boolean) (SweepResult :type "HitResult Structure (by ref)"))
  (cast `StaticMeshActor` OtherActor
    (:`then`
      (`self.K2_DestroyActor`))
    (:`CastFailed`
      (if (!= OtherActor (`self.GetOwner`))
        (bind _returnvalue (`CurseelBlueprintFunctionLibrary.GetCurseelASC` OtherActor))
        (`CurseelBlueprintFunctionLibrary.ApplyEffect` (make `GameplayEffectApplier` (`self.OwnerASC`) _returnvalue "Target" "/Game/Blueprints/GE_GenericDamage.GE_GenericDamage_C" (struct :`TagName` "Data.Damage") (`self.Damage`)))
        (`self.K2_DestroyActor`)))))

(fn `UserConstructionScript`)