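; Gameplay Ability for a generic attack that spawns a configurable AOE actor owned by the avatar.
; Once committed, it applies a cooldown effect with a random duration scaled by an avatar attribute, then spawns the AOE.
; The ability ends when the AOE or avatar is destroyed.
; Stunning the character destroys the AOE, as does destruction of the avatar.
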(event `self.K2_ActivateAbility`
  (bind _returnvalue (`self.GetAvatarActorFromActorInfo`))
  (add `Actor.OnDestroyed` _returnvalue (delegate `OnAvatarActorDestroyed`))
  (bind _ascharacter_base (cast `CharacterBase` _returnvalue)
    (:`then`
      (add `CharacterBase.OnCharacterStunned` _ascharacter_base (delegate `OnCharacterStunned_Event`)))
    (:`CastFailed`
      _))
  (bind _returnvalue_2 (`self.K2_CommitAbility`))
  (if _returnvalue_2
    (bind _spawnedaoe (`self.SpawnAOE` (`self.AttackAOE`)))
    (add `Actor.OnDestroyed` _spawnedaoe (delegate `OnAOE_Destroyed`))))

(event `OnAOE_Destroyed`
  (params (DestroyedActor :type "Actor Object Reference"))
  (`self.K2_EndAbility`))

(event `OnCharacterStunned_Event`
  (params (Character :type "CharacterBase Object Reference") (Stunned :type Boolean))
  (bind _aoe (`self.AOE`))
  (if Stunned
    (`/Engine/EditorBlueprintResources/StandardMacros.IsValid` _aoe
      (:`Is Valid`
        (`Actor.K2_DestroyActor` _aoe)))))

(event `OnAvatarActorDestroyed`
  (params (DestroyedActor :type "Actor Object Reference"))
  (bind _aoe (`self.AOE`))
  (`self.K2_EndAbility`)
  (`/Engine/EditorBlueprintResources/StandardMacros.IsValid` _aoe
    (:`Is Valid`
      (`Actor.K2_DestroyActor` _aoe))))

(fn `Get CDDuration`
  (returns (Duration :type "Float (single-precision)"))
  (return (* (`KismetMathLibrary.RandomFloatInRange` (`self.CD_MaxDuration`) (`self.CD_MinDuration`)) (`.ReturnValue` (`AbilitySystemBlueprintLibrary.GetFloatAttribute` (`self.GetAvatarActorFromActorInfo`) (struct :`AttributeName` "AttackSpeed" :`Attribute` "/Script/Curseel.AttributeSetBase:AttackSpeed" :`AttributeOwner` "/Script/CoreUObject.Class'\"/Script/Curseel.AttributeSetBase\"'"))))))

(fn `SpawnAOE`
  (params (AOE :type "Actor Class Reference"))
  (returns (SpawnedAOE :type "Actor Object Reference"))
  (bind _returnvalue (`AbilitySystemBlueprintLibrary.GetAbilitySystemComponent` (`self.GetAvatarActorFromActorInfo`)))
  (bind _returnvalue_2 (`AbilitySystemBlueprintLibrary.SetDuration` (`AbilitySystemComponent.MakeOutgoingSpec` _returnvalue "/Game/Blueprints/GE_DefaultGenericAttackCooldown.GE_DefaultGenericAttackCooldown_C" 0.0 (`AbilitySystemComponent.MakeEffectContext` _returnvalue)) (`self.Get CDDuration`)))
  (`AbilitySystemComponent.BP_ApplyGameplayEffectSpecToSelf` _returnvalue _returnvalue_2)
  (bind _returnvalue_3 (`|SpawnActorFromClass` (`local.AOE`) (`KismetMathLibrary.MakeTransform` (0.0 0.0 -89.0)) "Undefined" "MultiplyWithRoot" (`self.GetAvatarActorFromActorInfo`) null))
  (bind _output_get (set `self.AOE` _returnvalue_3))
  (return _output_get))