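; BP_PoisonManager spawns area-of-effect poison actors near the player's predicted position on a looping timer.
; The timer is paused right after BeginPlay creates it, and ToogleSpawn pauses or resumes it.
; Each spawn extrapolates the player's location from velocity, adds a random XY offset and clamps it within a range limit.
; Spawned BP_AOE_Poison actors are tracked in an array, which RemoveAllPoison destroys and clears.
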(event `RemoveAllPoison`
  (bind _poisons (`self.Poisons`))
  (for _array_element _poisons
    (`self.K2_DestroyActor` _array_element))
  (`KismetArrayLibrary.Array_Clear` _poisons))

(event `ToogleSpawn`
  (bind _spawnpoisontimer (`self.SpawnPoisonTimer`))
  (if (`KismetSystemLibrary.K2_IsTimerPausedHandle` _spawnpoisontimer)
    (`KismetSystemLibrary.K2_UnPauseTimerHandle` _spawnpoisontimer)
    (else
      (`KismetSystemLibrary.K2_PauseTimerHandle` _spawnpoisontimer))))

(event `self.ReceiveBeginPlay`
  (bind _returnvalue (`KismetSystemLibrary.K2_SetTimerDelegate` (delegate `SpawnPoison`) 5.0 true))
  (set `self.SpawnPoisonTimer` _returnvalue)
  (`self.ToogleSpawn`))

(event `SpawnPoison`
  (bind _returnvalue (`GameplayStatics.GetPlayerPawn` 0))
  (bind (_randomoffset_x _randomoffset_y) (`KismetMathLibrary.BreakVector` (`self.RandomOffset`)))
  (bind _rangelimit (`self.RangeLimit`))
  (bind _rangelimit_2 (`self.RangeLimit`))
  (bind (_returnvalue_x _returnvalue_y) (`KismetMathLibrary.BreakVector` (+ (* (`self.PredictionTime`) (`self.GetVelocity` _returnvalue)) (`self.K2_GetActorLocation` _returnvalue) (`KismetMathLibrary.MakeVector` (`KismetMathLibrary.RandomFloatInRange` (* -1.0 _randomoffset_x) _randomoffset_x) (`KismetMathLibrary.RandomFloatInRange` (* _randomoffset_y -1.0) _randomoffset_y)))))
  (bind _returnvalue_2 (`|SpawnActorFromClass` "/Game/Blueprints/BP_AOE_Poison.BP_AOE_Poison_C" (`KismetMathLibrary.MakeTransform` (`KismetMathLibrary.MakeVector` (`KismetMathLibrary.FClamp` _returnvalue_x (* _rangelimit_2 -1.0) _rangelimit_2) (`KismetMathLibrary.FClamp` _returnvalue_y (* _rangelimit -1.0) _rangelimit))) "AlwaysSpawn" "MultiplyWithRoot" null null))
  (`KismetArrayLibrary.Array_Add` (`self.Poisons`) _returnvalue_2))

(fn `UserConstructionScript`)