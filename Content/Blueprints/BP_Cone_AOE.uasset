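; Cone-shaped area-of-effect actor that builds its own procedural mesh and attaches to its owner on BeginPlay.
; Construction and BeginPlay generate a collidable triangle fan from an origin vertex, extending by Distance and adding paired vertices per Resolution step.
; BeginPlay applies the AOE material, snaps to the owner and activates the AOE.
; ActivateSnapshot extends the parent's behavior by setting the material's Hit parameter.
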(event `self.ReceiveBeginPlay`
  (`parent.ReceiveBeginPlay`)
  (`self.CreateProceduralAOE`)
  (`PrimitiveComponent.SetMaterial` (`self.ProceduralMesh`) 0 "/Game/Placeholder/MI_AOE.MI_AOE")
  (`self.K2_AttachToActor` (`self.GetOwner`) "None" "SnapToTarget" "SnapToTarget" "SnapToTarget")
  (`self.ActivateAOE`))

(event `self.DisplayTelegraph`)

(event `self.ActivateSnapshot`
  (`parent.ActivateSnapshot`)
  (`MeshComponent.SetScalarParameterValueOnMaterials` (`self.ProceduralMesh`) "Hit" 1.0))

(fn `ClearMesh`
  (`KismetArrayLibrary.Array_Clear` (`self.Vertices`))
  (`KismetArrayLibrary.Array_Clear` (`self.Triangles`))
  (return))

(fn `CreateProceduralAOE`
  (`self.ClearMesh`)
  (`|ExecutionSequence`
    (:`then_0`
      (`self.CreateVertices`))
    (:`then_1`
      (`self.CreateTriangles`))
    (:`then_2`
      (bind (_normals _tangents) (`KismetProceduralMeshLibrary.CalculateTangentsForMesh` (`self.Vertices`) (`self.Triangles`)))
      (`ProceduralMeshComponent.CreateMeshSection_LinearColor` :`self` (`self.ProceduralMesh`) :`Vertices` (`self.Vertices`) :`Triangles` (`self.Triangles`) :`Normals` _normals :`Tangents` _tangents :`bCreateCollision` true))))

(fn `CreateTriangles`
  (for _index (range (+ (`self.Resolution`) 1))
    (`|ExecutionSequence`
      (:`then_0`
        (`KismetArrayLibrary.Array_Add` (`self.Triangles`))
        (bind _returnvalue (+ (* _index 2) 2))
        (`KismetArrayLibrary.Array_Add` (`self.Triangles`) _returnvalue)
        (bind _returnvalue_2 (== _index 0))
        (`KismetArrayLibrary.Array_Add` (`self.Triangles`) (select `bool` _returnvalue_2 :`false` (- _returnvalue 2) :`true` 1)))
      (:`then_1`
        (`KismetArrayLibrary.Array_Add` (`self.Triangles`))
        (bind _returnvalue_3 (+ _returnvalue 1))
        (`KismetArrayLibrary.Array_Add` (`self.Triangles`) (select `bool` _returnvalue_2 :`false` (- _returnvalue_3 2) :`true` 1))
        (`KismetArrayLibrary.Array_Add` (`self.Triangles`) _returnvalue_3)))))

(fn `CreateVertices`
  (bind _distance (`self.Distance`))
  (bind _resolution (`self.Resolution`))
  (bind _vertices (`self.Vertices`))
  (`KismetArrayLibrary.Array_Add` (`self.Vertices`))
  (`KismetArrayLibrary.Array_Add` (`self.Vertices`) (`KismetMathLibrary.MakeVector` (`self.Distance`)))
  (for _index (range (+ _resolution 1))
    (bind _returnvalue (`KismetMathLibrary.DegreesToRadians` (* (* (select `bool` (== _resolution 0) :`false` (/ (`KismetMathLibrary.Conv_IntToDouble` _index) (`KismetMathLibrary.Conv_IntToDouble` _resolution)) :`true` 1.0) (`self.Angle(Degrees)`)) 0.5)))
    (bind _returnvalue_2 (* (`KismetMathLibrary.Cos` _returnvalue) _distance))
    (bind _returnvalue_3 (* (`KismetMathLibrary.Sin` _returnvalue) _distance))
    (`KismetArrayLibrary.Array_Add` _vertices (`KismetMathLibrary.MakeVector` _returnvalue_2 _returnvalue_3))
    (`KismetArrayLibrary.Array_Add` _vertices (`KismetMathLibrary.MakeVector` _returnvalue_2 (* _returnvalue_3 -1.0)))))

(fn `UserConstructionScript`
  (`self.CreateProceduralAOE`))