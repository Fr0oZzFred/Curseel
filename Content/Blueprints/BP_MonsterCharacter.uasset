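; AI monster character that detects the player's BP_Wheel pawn, attacks it at close range and destroys itself on death.
; PawnSensing flags the sighting on the blackboard and enables Tick, which sets the Attack key within AttackRange and prints debug HP.
; Attack activates the first Gameplay Ability and turns to face the player; EndAttack clears the state.
; The construction script optionally adds a sphere visualizing attack range.
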(event `self.ReceiveBeginPlay`
  (add `self.OnCharacterDied` (delegate `OnCharacterDied_Event`)))

(event `OnCharacterDied_Event` :!signature `self.OnCharacterDied`
  (params (Character :type "CharacterBase Object Reference"))
  (`self.K2_DestroyActor`))

(event `self.ReceiveTick`
  (params (DeltaSeconds :type "Float (single-precision)"))
  (`self.TryAttack`)
  (`KismetSystemLibrary.PrintString` (`KismetStringLibrary.Concat_StrStr` (`KismetSystemLibrary.GetDisplayName` self) " HP: " (`KismetStringLibrary.Conv_DoubleToString` (`self.GetHealth`))) true true (struct :`G` 0.66 :`B` 1.0 :`A` 1.0) 0.0))

(event `self.PawnSensing.OnSeePawn`
  (params (Pawn :type "Pawn Object Reference"))
  (bind _asbp_wheel (cast `/Game/Blueprints/Bp_Wheel` Pawn))
  (set `self.PlayerWheel` _asbp_wheel)
  (`BlackboardComponent.SetValueAsBool` (`AIBlueprintHelperLibrary.GetBlackboard` null) "HasSeenPlayer" true)
  (`self.SetActorTickEnabled` true))

(event `TryAttack`
  (if (and (not (`self.Attacking`)) (< (`KismetMathLibrary.Abs` (`KismetMathLibrary.VSize` (- (`self.K2_GetActorLocation` (`self.PlayerWheel`)) (`self.K2_GetActorLocation` self)))) (`self.AttackRange`)))
    (`BlackboardComponent.SetValueAsBool` (`AIBlueprintHelperLibrary.GetBlackboard` null) "Attack" true)))

(event `Attack`
  (bind _returnvalue (`KismetAnimationLibrary.K2_LookAt` (`self.GetTransform`) (`self.K2_GetActorLocation` (`self.PlayerWheel`)) (1.0 0.0 0.0)))
  (if (not (`self.Attacking`))
    (bind _returnvalue_2 (`AbilitySystemComponent.TryActivateAbilityByClass` (`self.HardRefAbilitySystemComponent`) (`|GetArrayItem` (`self.CharacterAbilities`)) true))
    (bind _output_get (set `self.Attacking` _returnvalue_2))
    (if _output_get
      (`self.K2_SetActorTransform` (`KismetMathLibrary.MakeTransform` (.location _returnvalue) (`KismetMathLibrary.MakeRotator` 0.0 0.0 (.yaw (.rotation _returnvalue))) (.scale _returnvalue))))))

(event `EndAttack`
  (bind _returnvalue (`AIBlueprintHelperLibrary.GetBlackboard` null))
  (`/Engine/EditorBlueprintResources/StandardMacros.IsValid` _returnvalue
    (:`Is Valid`
      (`BlackboardComponent.SetValueAsBool` _returnvalue "Attack" false)
      (set `self.Attacking` false))))

(fn `UserConstructionScript`
  (bind _debugsphere (`self.DebugSphere`))
  (bind _debugsphere_2 (`self.DebugSphere`))
  (if (`self.DebugAttackRange`)
    (`/Engine/EditorBlueprintResources/StandardMacros.IsValid` (`self.DebugSphere`)
      (:`Is Not Valid`
        (bind _returnvalue (`AddComponent|NODE_AddSphereComponent-0` :`bManualAttachment` true))
        (set `self.DebugSphere` _returnvalue)
        (`|ExecutionSequence`
          (:`then_0`
            (`PrimitiveComponent.SetCollisionEnabled` _debugsphere "NoCollision")
            (`SphereComponent.SetSphereRadius` _debugsphere (`self.AttackRange`) false))
          (:`then_1`
            (`SceneComponent.SetHiddenInGame` _debugsphere_2 false false)
            (`SceneComponent.K2_AttachToComponent` _debugsphere_2 (`self.Mesh`) "None" "SnapToTarget" "SnapToTarget" "KeepWorld" true)))))
    (else
      (`/Engine/EditorBlueprintResources/StandardMacros.IsValid` (`self.DebugSphere`)
        (:`Is Valid`
          (`ActorComponent.K2_DestroyComponent` (`self.DebugSphere`)))))))