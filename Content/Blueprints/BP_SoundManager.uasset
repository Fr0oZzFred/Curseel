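; Sound manager that plays music themes and one-shot 2D effects, registering itself with the game mode on BeginPlay.
; It starts an optional entry theme, and a FlipFlop toggle alternates battle and dungeon themes through FadeToTheme, which fades out the current track while fading in the next.
; The chosen and fire sound events spawn a sound only when their stored audio component is invalid, preventing overlapping copies.
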(event `self.ReceiveBeginPlay`
  (bind _entrytheme (`self.EntryTheme`))
  (message `/Game/GameModes/BPI_CurseelGM.SetSoundManager` (`GameplayStatics.GetGameMode`) self)
  (`/Engine/EditorBlueprintResources/StandardMacros.IsValid` _entrytheme
    (:`Is Valid`
      (bind _returnvalue (`GameplayStatics.SpawnSound2D` _entrytheme 1.0 1.0 0.0 null))
      (set `self.CurrentTheme` _returnvalue))))

(event `ToogleBattleTheme`
  (bind _isa (`/Engine/EditorBlueprintResources/StandardMacros.FlipFlop`)
    (:`A`
      _)
    (:`B`
      _))
  (`self.FadeToTheme` (select `bool` _isa :`false` (`self.DungeonTheme`) :`true` (`self.BattleTheme`))))

(event `PlayChosenSoundOnce`
  (`/Engine/EditorBlueprintResources/StandardMacros.IsValid` (`self.ChosenSound`)
    (:`Is Not Valid`
      (bind _returnvalue (`GameplayStatics.SpawnSound2D` "/Game/Placeholder/Audio/UI_pack_1/MENU_B_Back.MENU_B_Back" 1.0 1.0 0.0 null))
      (set `self.ChosenSound` _returnvalue))))

(event `PlayFireSoundOnce`
  (`/Engine/EditorBlueprintResources/StandardMacros.IsValid` (`self.FireSound`)
    (:`Is Not Valid`
      (bind _returnvalue (`GameplayStatics.SpawnSound2D` "/Game/Placeholder/Audio/Magic_SFX_Preview_Pack/Fire_impact_1.Fire_impact_1" 1.0 1.0 0.0 null))
      (set `self.FireSound` _returnvalue))))

(fn `CurrentThemeFadeOut`
  (`AudioComponent.FadeOut` (`self.CurrentTheme`) (* (`self.FadeDuration`) 0.5) 0.0 "Linear"))

(fn `FadeToTheme`
  (params (Sound :type "SoundBase Object Reference"))
  (`AudioComponent.FadeOut` (`self.CurrentTheme`) (* (`self.FadeDuration`) 0.5) 0.0 "Linear")
  (bind _returnvalue (`GameplayStatics.SpawnSound2D` (`local.Sound`) 1.0 1.0 0.0 null))
  (bind _output_get (set `self.CurrentTheme` _returnvalue))
  (`AudioComponent.FadeIn` _output_get (`self.FadeDuration`) 1.0 0.0 "Linear"))

(fn `UserConstructionScript`)