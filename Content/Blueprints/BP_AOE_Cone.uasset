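; Cone-shaped area attack, a child AOE actor that deals GAS damage to characters it catches and slows monsters.
; It builds a procedural fan mesh from radius and angle, with material parameters animating the telegraph and flagging the hit.
; It follows its owner until the telegraph ends, then detaches and spawns matching VFX.
; Collision checks narrow sphere overlaps by angle, hitting each character once with set-by-caller damage.
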(event `OnCharacterHit_Event` :!signature `self.OnCharacterHit`
  (params (HitCharacter :type "CharacterBase Object Reference"))
  (bind _asbp_monster_character (cast `/Game/Monsters/BP_MonsterCharacter` HitCharacter))
  (bind _returnvalue (`AbilitySystemBlueprintLibrary.GetAbilitySystemComponent` _asbp_monster_character))
  (`AbilitySystemComponent.BP_ApplyGameplayEffectSpecToSelf` _returnvalue (`AbilitySystemComponent.MakeOutgoingSpec` _returnvalue "/Game/Monsters/GE_Slow.GE_Slow_C" 0.0 (`AbilitySystemComponent.MakeEffectContext` _returnvalue))))

(event `self.ReceiveBeginPlay`
  (`parent.ReceiveBeginPlay`)
  (`self.CreateProceduralAOE`)
  (`PrimitiveComponent.SetMaterial` (`self.ProceduralMesh`) 0 "/Game/Placeholder/MI_AOE.MI_AOE")
  (`self.K2_AttachToActor` (`self.GetOwner`) "None" "KeepRelative" "KeepRelative" "SnapToTarget")
  (`SphereComponent.SetSphereRadius` (`self.Sphere`) (`self.Radius`) true)
  (`self.ActivateAOE`)
  (add `self.OnTelegraphEnd` (delegate `OnTelegraphEnd_Event`))
  (add `self.OnCharacterHit` (delegate `OnCharacterHit_Event`)))

(event `OnTelegraphEnd_Event`
  (bind (_returnvalue_location _returnvalue_rotation _returnvalue_scale) (`KismetMathLibrary.BreakTransform` (`self.GetTransform`)))
  (bind _vfx (`self.VFX`))
  (`self.K2_DetachFromActor` "KeepWorld" "KeepWorld" "KeepWorld")
  (`/Engine/EditorBlueprintResources/StandardMacros.IsValid` _vfx
    (:`Is Valid`
      (bind _returnvalue (`NiagaraFunctionLibrary.SpawnSystemAtLocation` _vfx _returnvalue_location _returnvalue_rotation _returnvalue_scale))
      (`FXSystemComponent.SetFloatParameter` _returnvalue "Radius" (`self.Radius`))
      (`FXSystemComponent.SetFloatParameter` _returnvalue "Angle" (`self.Angle(Degrees)`)))))

(event `self.DisplayTelegraph`
  (`TimelineComponent.SetPlayRate` (`self.TelegraphAnimation`) (/ 1.0 (`self.TelegraphDuration`)))
  (bind (_direction _progression) (`Timeline|TelegraphAnimation` :!via `PlayFromStart`)
    (:`Update`
      (`MeshComponent.SetScalarParameterValueOnMaterials` (`self.ProceduralMesh`) "Progression" _progression))))

(event `self.ActivateSnapshot`
  (`parent.ActivateSnapshot`)
  (`MeshComponent.SetScalarParameterValueOnMaterials` (`self.ProceduralMesh`) "Hit" 1.0))

(event `self.CheckForCharactersCollision`
  (bind _vertices (`self.Vertices`))
  (bind _returnvalue (`KismetArrayLibrary.Array_LastIndex` _vertices))
  (bind (_output_x _output_y) (`KismetMathLibrary.BreakVector` (`|GetArrayItem` _vertices _returnvalue)))
  (bind (_output_x_2 _output_y_2) (`KismetMathLibrary.BreakVector` (`|GetArrayItem` _vertices (- _returnvalue 1))))
  (`parent.CheckForCharactersCollision`)
  (for _array_element (`PrimitiveComponent.GetOverlappingActors` (`self.Sphere`) (`self.TargetFilter`))
    (bind (_returnvalue_x _returnvalue_y) (`KismetMathLibrary.BreakVector` (`KismetMathLibrary.InverseTransformLocation` (`self.GetTransform`) (`self.K2_GetActorLocation` _array_element))))
    (bind _returnvalue_2 (`KismetMathLibrary.Atan2` _returnvalue_y _returnvalue_x))
    (if (and (and (< (`KismetMathLibrary.Atan2` _output_y _output_x) _returnvalue_2) (> (`KismetMathLibrary.Atan2` _output_y_2 _output_x_2) _returnvalue_2)) (== (`KismetArrayLibrary.Array_Find` (`self.TouchedActors`) _array_element) -1))
      (bind _ascharacter_base (cast `CharacterBase` _array_element))
      (`KismetArrayLibrary.Array_Add` (`self.TouchedActors`) _ascharacter_base)
      (bind _returnvalue_3 (`AbilitySystemBlueprintLibrary.GetAbilitySystemComponent` _ascharacter_base))
      (bind _returnvalue_4 (`AbilitySystemBlueprintLibrary.AssignTagSetByCallerMagnitude` (`AbilitySystemComponent.MakeOutgoingSpec` _returnvalue_3 "/Game/Blueprints/GE_GenericDamage.GE_GenericDamage_C" 0.0 (`AbilitySystemComponent.MakeEffectContext` _returnvalue_3)) (struct :`TagName` "Data.Damage") (`self.Damage`)))
      (`AbilitySystemComponent.BP_ApplyGameplayEffectSpecToSelf` _returnvalue_3 _returnvalue_4)
      (`self.OnCharacterHit` _ascharacter_base))))

(fn `ClearMesh`
  (`KismetArrayLibrary.Array_Clear` (`self.Vertices`))
  (`KismetArrayLibrary.Array_Clear` (`self.Triangles`))
  (`KismetArrayLibrary.Array_Clear` (`self.UVs`))
  (return))

(fn `CreateProceduralAOE`
  (`self.ClearMesh`)
  (`|ExecutionSequence`
    (:`then_0`
      (`self.CreateVertices`))
    (:`then_1`
      (`self.CreateTriangles`))
    (:`then_2`
      (`self.CreateUVs`))
    (:`then_3`
      (bind (_normals _tangents) (`KismetProceduralMeshLibrary.CalculateTangentsForMesh` (`self.Vertices`) (`self.Triangles`) (`self.UVs`)))
      (`ProceduralMeshComponent.CreateMeshSection_LinearColor` :`self` (`self.ProceduralMesh`) :`Vertices` (`self.Vertices`) :`Triangles` (`self.Triangles`) :`Normals` _normals :`UV0` (`self.UVs`) :`Tangents` _tangents))))

(fn `CreateTriangles`
  (for _index (range (+ (`self.Resolution`) 1))
    (`|ExecutionSequence`
      (:`then_0`
        (`KismetArrayLibrary.Array_Add` (`self.Triangles`))
        (bind _returnvalue (+ (* _index 2) 2))
        (`KismetArrayLibrary.Array_Add` (`self.Triangles`) _returnvalue)
        (bind _returnvalue_2 (== _index 0))
        (`KismetArrayLibrary.Array_Add` (`self.Triangles`) (select `bool` _returnvalue_2 :`false` (- _returnvalue 2) :`true` 1)))
      (:`then_1`
        (`KismetArrayLibrary.Array_Add` (`self.Triangles`))
        (bind _returnvalue_3 (+ _returnvalue 1))
        (`KismetArrayLibrary.Array_Add` (`self.Triangles`) (select `bool` _returnvalue_2 :`false` (- _returnvalue_3 2) :`true` 1))
        (`KismetArrayLibrary.Array_Add` (`self.Triangles`) _returnvalue_3)))))

(fn `CreateUVs`
  (`KismetArrayLibrary.Array_Add` (`self.UVs`))
  (for _ (range 1 (+ (`KismetArrayLibrary.Array_LastIndex` (`self.Vertices`)) 1))
    (`KismetArrayLibrary.Array_Add` (`self.UVs`) (0.0 1.0))))

(fn `CreateVertices`
  (bind _radius (`self.Radius`))
  (bind _resolution (`self.Resolution`))
  (bind _vertices (`self.Vertices`))
  (`KismetArrayLibrary.Array_Add` (`self.Vertices`))
  (`KismetArrayLibrary.Array_Add` (`self.Vertices`) (`KismetMathLibrary.MakeVector` (`self.Radius`)))
  (for _index (range (+ _resolution 1))
    (bind _returnvalue (`KismetMathLibrary.DegreesToRadians` (* (* (select `bool` (== _resolution 0) :`false` (/ (`KismetMathLibrary.Conv_IntToDouble` _index) (`KismetMathLibrary.Conv_IntToDouble` _resolution)) :`true` 1.0) (`self.Angle(Degrees)`)) 0.5)))
    (bind _returnvalue_2 (* (`KismetMathLibrary.Cos` _returnvalue) _radius))
    (bind _returnvalue_3 (* (`KismetMathLibrary.Sin` _returnvalue) _radius))
    (`KismetArrayLibrary.Array_Add` _vertices (`KismetMathLibrary.MakeVector` _returnvalue_2 _returnvalue_3))
    (`KismetArrayLibrary.Array_Add` _vertices (`KismetMathLibrary.MakeVector` _returnvalue_2 (* _returnvalue_3 -1.0)))))

(fn `UserConstructionScript`
  (`self.CreateProceduralAOE`))