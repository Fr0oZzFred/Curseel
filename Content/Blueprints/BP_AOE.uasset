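; Area-of-effect actor skeleton that runs a timed telegraph, then a snapshot window, then destroys itself.
; Collision starts disabled; ActivateAOE waits out the telegraph, enables collision, fires OnTelegraphEnd and destroys the actor after the snapshot duration.
; During the snapshot, a DelayUntilNextTick loop calls CheckForCharactersCollision every frame until destruction.
; That check is an empty event, and the telegraph display only prints a not-implemented message.
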(event `self.ReceiveBeginPlay`
  (`self.SetActorEnableCollision` self false))

(event `ActivateAOE`
  (`self.DisplayTelegraph`)
  (`KismetSystemLibrary.Delay` (`self.TelegraphDuration`))
  (`self.ActivateSnapshot`)
  (`self.OnTelegraphEnd`)
  (`KismetSystemLibrary.Delay` (`self.SnapshotDuration`))
  (`self.K2_DestroyActor`))

(event `DisplayTelegraph`
  (`KismetSystemLibrary.PrintString` "Need to Implement Telegraph"))

(event `ActivateSnapshot`
  (`self.SetActorEnableCollision` self true)
  (`KismetSystemLibrary.DelayUntilNextTick` :!label _label) ; Tick every frame until destroy event
  (`self.CheckForCharactersCollision`)
  (goto _label))

(event `CheckForCharactersCollision`)

(fn `UserConstructionScript`)