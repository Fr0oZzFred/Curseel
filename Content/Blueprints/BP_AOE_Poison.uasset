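; BP_AOE_Poison is an area-of-effect hazard that damages characters inside a radius-scaled sphere.
; It activates on BeginPlay, extending parent AOE logic with a timeline-driven material telegraph and a material hit flag at snapshot.
; Its collision check hits each overlapping target once, applying GE_GenericDamage via SetByCaller, reduced by the player's BP_OldWheel shield, then depletes that shield and fires a hit callback.
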(event `self.ReceiveBeginPlay`
  (`parent.ReceiveBeginPlay`)
  (`SceneComponent.SetRelativeScale3D` (`self.AOE`) (`KismetMathLibrary.Conv_DoubleToVector` (* (`self.Radius`) 0.01)))
  (`SphereComponent.SetSphereRadius` (`self.Sphere`) (`self.Radius`) true)
  (`self.ActivateAOE`))

(event `self.DisplayTelegraph`
  (`TimelineComponent.SetPlayRate` (`self.TelegraphAnimation`) (/ 1.0 (`self.TelegraphDuration`)))
  (bind (_direction _progression) (`Timeline|TelegraphAnimation` :!via `PlayFromStart`)
    (:`Update`
      (`MeshComponent.SetScalarParameterValueOnMaterials` (`self.AOE`) "Progression" _progression))))

(event `self.ActivateSnapshot`
  (`parent.ActivateSnapshot`)
  (`MeshComponent.SetScalarParameterValueOnMaterials` (`self.AOE`) "Hit" 1.0))

(event `self.CheckForCharactersCollision`
  (bind _asbp_old_wheel (cast `/Game/Wheel/BP_OldWheel` (`GameplayStatics.GetPlayerPawn` 0) :!pure true))
  (`parent.CheckForCharactersCollision`)
  (for _array_element (`PrimitiveComponent.GetOverlappingActors` (`self.Sphere`) (`self.TargetFilter`))
    (if (== (`KismetArrayLibrary.Array_Find` (`self.TouchedActors`) _array_element) -1)
      (bind _ascharacter_base (cast `CharacterBase` _array_element))
      (`KismetArrayLibrary.Array_Add` (`self.TouchedActors`) _ascharacter_base)
      (bind _returnvalue (`AbilitySystemBlueprintLibrary.GetAbilitySystemComponent` _ascharacter_base))
      (bind _returnvalue_2 (`AbilitySystemBlueprintLibrary.AssignTagSetByCallerMagnitude` (`AbilitySystemComponent.MakeOutgoingSpec` _returnvalue "/Game/Blueprints/GE_GenericDamage.GE_GenericDamage_C" 0.0 (`AbilitySystemComponent.MakeEffectContext` _returnvalue)) (struct :`TagName` "Data.Damage") (- (`self.Damage`) (`/Game/Wheel/BP_OldWheel.Shield` _asbp_old_wheel))))
      (`AbilitySystemComponent.BP_ApplyGameplayEffectSpecToSelf` _returnvalue _returnvalue_2)
      (`/Game/Wheel/BP_OldWheel.UpdateShield` _asbp_old_wheel (* (`self.Damage`) -1.0))
      (`self.OnCurseelActorHit` _array_element))))

(fn `UserConstructionScript`
  (`parent.UserConstructionScript`))