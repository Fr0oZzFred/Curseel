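; BP_BoostsVendor is a world vendor that opens the boost shop menu when the player's wheel interacts nearby.
; On BeginPlay it caches the player BP_Wheel and binds to its OnInteract event.
; A sphere overlap toggles an Interact prompt for the wheel.
; Interacting while overlapping pushes W_BoostMenuVendor onto the HUD's GameMenu layer stack.
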(event `self.ReceiveBeginPlay`
  (bind _asbp_wheel (cast `/Game/Wheel/BP_Wheel` (`GameplayStatics.GetPlayerPawn` 0)))
  (bind _output_get (set `self.Wheel` _asbp_wheel))
  (add `WheelPawn.OnInteract` _output_get (delegate `OnInteract_Event`)))

(event `OnInteract_Event`
  (if (`self.IsOverlappingWheel`)
    (bind _pushedwidget (`/Game/UI/W_Overall_UI_Layout.PushWidgetToLayerStack` (`/Game/GameModes/InGame/HUD_InGame.Overall_UI_Layout` (`/Game/GameModes/InGame/GM_InGame.HUD` (cast `/Game/GameModes/InGame/GM_InGame` (`GameplayStatics.GetGameMode`) :!pure true))) (struct :`TagName` "UI.Layer.GameMenu") "/Game/Boosts/UI/W_BoostMenuVendor.W_BoostMenuVendor_C"))
    (cast `/Game/Boosts/UI/W_BoostMenu` _pushedwidget)))

(event `self.Sphere.OnComponentBeginOverlap`
  (params (OverlappedComponent :type "PrimitiveComponent Object Reference") (OtherActor :type "Actor Object Reference") (OtherComp :type "PrimitiveComponent Object Reference") (OtherBodyIndex :type Integer) (bFromSweep :type Boolean) (SweepResult :type "HitResult Structure (by ref)"))
  (if (== OtherActor (`self.Wheel`))
    (`SceneComponent.SetVisibility` (`self.Interact`) true false)))

(event `self.Sphere.OnComponentEndOverlap`
  (params (OverlappedComponent :type "PrimitiveComponent Object Reference") (OtherActor :type "Actor Object Reference") (OtherComp :type "PrimitiveComponent Object Reference") (OtherBodyIndex :type Integer))
  (if (== OtherActor (`self.Wheel`))
    (`SceneComponent.SetVisibility` (`self.Interact`) false false)))

(fn `IsOverlappingWheel`
  (returns (ReturnValue :type Boolean))
  (return (`PrimitiveComponent.IsOverlappingActor` (`self.Sphere`) (`self.Wheel`))))

(fn `UserConstructionScript`)