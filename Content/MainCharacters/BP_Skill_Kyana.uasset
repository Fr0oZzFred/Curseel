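; Kyana's skill actor: a timed ring of orbiting spheres that damages monsters on overlap.
; SpawnSpheres spaces sphere colliders evenly around a circle, each with attached Niagara VFX, and runs at construction and BeginPlay, destroying previous components first.
; Tick yaws the root to spin the ring, and lifespan ends it after Duration.
; Overlapping a BP_MonsterCharacter applies GE_GenericDamage with SetByCaller damage and spawns a hit effect.
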(event `self.ReceiveBeginPlay`
  (`self.SpawnSpheres`)
  (`self.SetLifeSpan` (`self.Duration`)))

(event `self.ReceiveTick`
  (params (DeltaSeconds :type "Float (single-precision)"))
  (`SceneComponent.K2_AddRelativeRotation` (`self.DefaultSceneRoot`) (`KismetMathLibrary.MakeRotator` 0.0 0.0 (* DeltaSeconds (`self.Speed`))) false false))

(event `self.ReceiveActorBeginOverlap`
  (params (OtherActor :type "Actor Object Reference"))
  (bind _asbp_monster_character (cast `/Game/Blueprints/BP_MonsterCharacter` OtherActor))
  (bind _returnvalue (`AbilitySystemBlueprintLibrary.GetAbilitySystemComponent` _asbp_monster_character))
  (bind _returnvalue_2 (`AbilitySystemBlueprintLibrary.AssignTagSetByCallerMagnitude` (`AbilitySystemComponent.MakeOutgoingSpec` _returnvalue "/Game/Blueprints/GE_GenericDamage.GE_GenericDamage_C" 0.0 (`AbilitySystemComponent.MakeEffectContext` _returnvalue)) (struct :`TagName` "Data.Damage") (`self.Damage`)))
  (`AbilitySystemComponent.BP_ApplyGameplayEffectSpecToSelf` _returnvalue _returnvalue_2)
  (`NiagaraFunctionLibrary.SpawnSystemAtLocation` "/Game/Placeholder/VFX_Skill_Kyana_2.VFX_Skill_Kyana_2" (`self.K2_GetActorLocation` _asbp_monster_character)))

(fn `SpawnSpheres`
  (bind _spherenumber (`self.SphereNumber`))
  (bind _radius (`self.Radius`))
  (`|ExecutionSequence`
    (:`then_0`
      (for (_array_element _array_index) (`self.Spheres`)
        (`|ExecutionSequence`
          (:`then_0`
            (`/Engine/EditorBlueprintResources/StandardMacros.IsValid` _array_element
              (:`Is Valid`
                (`ActorComponent.K2_DestroyComponent` _array_element))))
          (:`then_1`
            (bind _output (`|GetArrayItem` (`self.VFXs`) _array_index))
            (`/Engine/EditorBlueprintResources/StandardMacros.IsValid` _output
              (:`Is Valid`
                (`ActorComponent.K2_DestroyComponent` _output)))))))
    (:`then_1`
      (for _index (range (+ _spherenumber 1))
        (bind _returnvalue (* (/ (`KismetMathLibrary.Conv_IntToDouble` _index) (`KismetMathLibrary.Conv_IntToDouble` _spherenumber)) (`KismetMathLibrary.GetTAU`)))
        (bind _returnvalue_2 (`AddComponent|NODE_AddSphereComponent-0` :`RelativeTransform` (`KismetMathLibrary.MakeTransform` (`KismetMathLibrary.MakeVector` (* (`KismetMathLibrary.Cos` _returnvalue) _radius) (* _radius (`KismetMathLibrary.Sin` _returnvalue))))))
        (`SphereComponent.SetSphereRadius` _returnvalue_2 50.0 true)
        (`KismetArrayLibrary.Array_Add` (`self.Spheres`) _returnvalue_2)
        (bind _returnvalue_3 (`NiagaraFunctionLibrary.SpawnSystemAttached` "/Game/Placeholder/VFX_Skill_Kyana.VFX_Skill_Kyana" _returnvalue_2 "None" (0.0 0.0 0.0) (struct) "SnapToTargetIncludingScale"))
        (`KismetArrayLibrary.Array_Add` (`self.VFXs`) _returnvalue_3)))))

(fn `UserConstructionScript`
  (`self.SpawnSpheres`))