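; Kyana's area-of-effect Blueprint, extending a parent that supplies the effect logic.
; On BeginPlay it plays a swing sound, then halves Damage if its owning BP_Wheel's current character index is not 1.
; Each ApplyEffect call runs the parent logic and then plays a 2D feedback sound.
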(event `self.ReceiveBeginPlay`
  (`parent.ReceiveBeginPlay`)
  (`GameplayStatics.PlaySound2D` "/Game/Placeholder/Audio/RPG_Sound_Pack/battle/swing3.swing3" 1.0 1.0 0.0 null null)
  (bind _asbp_wheel (cast `/Game/Wheel/BP_Wheel` (`self.GetOwner`)))
  (if (not (== (`WheelPawn.CurrentCharacterIndex` _asbp_wheel) 1))
    (bind _output_get (set `self.Damage` (* (stale _output_get) 0.5)))))

(event `self.ApplyEffect`
  (params (Actor :type "Actor Object Reference") (TouchedASC :type "AbilitySystemComponent Object Reference"))
  (`parent.ApplyEffect` Actor TouchedASC)
  (`GameplayStatics.PlaySound2D` "/Game/Placeholder/Audio/RPG_Sound_Pack/interface/interface2.interface2" 1.0 1.0 0.0 null null))

(fn `UserConstructionScript`
  (`parent.UserConstructionScript`))