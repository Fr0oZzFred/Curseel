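; Gameplay ability for Tolg's skill in the old character design, buffing the whole party at once.
; On a successful commit, it reads the Characters list from the avatar's owning BP_OldWheel.
; Each character gets health and damage-buff gameplay effects applied through its own ability system component.
; A health VFX is attached to the wheel's root, then the ability ends; a failed commit does nothing.
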(event `self.K2_ActivateAbility`
  (bind _returnvalue (`Actor.GetOwner` (`self.GetAvatarActorFromActorInfo`)))
  (bind _returnvalue_2 (`self.K2_CommitAbility`))
  (if _returnvalue_2
    (for _array_element (`/Game/Wheel/BP_OldWheel.Characters` (cast `/Game/Wheel/BP_OldWheel` _returnvalue :!pure true))
      (`|ExecutionSequence`
        (:`then_0`
          (bind _returnvalue_3 (`AbilitySystemBlueprintLibrary.GetAbilitySystemComponent` _array_element))
          (`AbilitySystemComponent.BP_ApplyGameplayEffectSpecToSelf` _returnvalue_3 (`AbilitySystemComponent.MakeOutgoingSpec` _returnvalue_3 "/Game/MainCharacters/OldDesign/GE_Skill_Health_Tolg.GE_Skill_Health_Tolg_C" 0.0 (`AbilitySystemComponent.MakeEffectContext` _returnvalue_3))))
        (:`then_1`
          (`AbilitySystemComponent.BP_ApplyGameplayEffectSpecToSelf` _returnvalue_3 (`AbilitySystemComponent.MakeOutgoingSpec` _returnvalue_3 "/Game/MainCharacters/OldDesign/GE_Skill_DamageBuff_Tolg.GE_Skill_DamageBuff_Tolg_C" 0.0 (`AbilitySystemComponent.MakeEffectContext` _returnvalue_3))))))
    (`NiagaraFunctionLibrary.SpawnSystemAttached` "/Game/Placeholder/VFX_Skill_Health_Tolg.VFX_Skill_Health_Tolg" (`Actor.RootComponent` _returnvalue) "None" (0.0 0.0 0.0) (struct) "SnapToTargetIncludingScale" true)
    (`self.K2_EndAbility`)))