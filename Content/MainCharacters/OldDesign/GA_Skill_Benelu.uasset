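; Gameplay ability for Benelu's skill in the old design, granting damage reduction to every character on the owning BP_OldWheel.
; On a successful commit, it applies GE_Skill_DMGReduction_Benelu to each character through that character's own ability system component.
; It waits for the last applied effect's total duration, then spawns BP_Skill_Benelu at the wheel's location and ends.
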(event `self.K2_ActivateAbility`
  (bind _returnvalue (`self.K2_CommitAbility`))
  (if _returnvalue
    (for _array_element (`/Game/Wheel/BP_OldWheel.Characters` (cast `/Game/Wheel/BP_OldWheel` (`Actor.GetOwner` (`self.GetAvatarActorFromActorInfo`)) :!pure true))
      (bind _returnvalue_2 (`AbilitySystemBlueprintLibrary.GetAbilitySystemComponent` _array_element))
      (bind _returnvalue_3 (`AbilitySystemComponent.BP_ApplyGameplayEffectSpecToSelf` _returnvalue_2 (`AbilitySystemComponent.MakeOutgoingSpec` _returnvalue_2 "/Game/MainCharacters/OldDesign/GE_Skill_DMGReduction_Benelu.GE_Skill_DMGReduction_Benelu_C" 0.0 (`AbilitySystemComponent.MakeEffectContext` _returnvalue_2))))
      (bind _returnvalue_4 (`AbilitySystemBlueprintLibrary.GetActiveGameplayEffectTotalDuration` _returnvalue_3)))
    (`KismetSystemLibrary.Delay` _returnvalue_4)
    (`|SpawnActorFromClass` "/Game/MainCharacters/OldDesign/BP_Skill_Benelu.BP_Skill_Benelu_C" (`KismetMathLibrary.MakeTransform` (`Actor.K2_GetActorLocation` (`Actor.GetOwner` (`self.GetAvatarActorFromActorInfo`)))) "Undefined" "MultiplyWithRoot" null null)
    (`self.K2_EndAbility`)))