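; Kyana's attack gameplay ability from the old character design, which turns cone AOE hits into combo on the player.
; It overrides only the parent's OnAOEDestroyed event, leaving activation and ending to the parent class.
; When a BP_AOE_Cone is destroyed, its touched-actor count goes to AddCombo on the BP_OldWheel player pawn, then the parent handler runs.
; A failed cone cast skips both steps, including the parent call.
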(event `self.OnAOE_Destroyed`
  (params (DestroyedActor :type "Actor Object Reference"))
  (bind _asbp_aoe_cone (cast `/Game/Blueprints/BP_AOE_Cone` DestroyedActor))
  (`/Game/Wheel/BP_OldWheel.AddCombo` (cast `/Game/Wheel/BP_OldWheel` (`GameplayStatics.GetPlayerPawn` 0) :!pure true) (`KismetArrayLibrary.Array_Length` (`/Game/Blueprints/BP_AOE_Cone.TouchedActors` _asbp_aoe_cone)))
  (`parent.OnAOE_Destroyed` DestroyedActor))