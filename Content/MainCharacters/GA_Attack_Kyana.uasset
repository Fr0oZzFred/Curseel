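; Gameplay ability blueprint for Kyana's attack, extending a parent attack ability that handles activation and area-of-effect behavior.
; When the AOE is destroyed it only forwards to the parent handler; activation and end overrides are disabled.
; A disconnected snippet would add the cone AOE's touched-actor count to the player BP_Wheel's combo, but it never runs.
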(event `self.OnAOE_Destroyed`
  (params (DestroyedActor :type "Actor Object Reference"))
  (`parent.OnAOE_Destroyed` DestroyedActor))