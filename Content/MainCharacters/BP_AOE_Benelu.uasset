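; Benelu's area-of-effect attack actor, which steals shield from characters it touches and tints its visual blue.
; On spawn it plays a swing sound and halves the steal amount when the owning BP_Wheel's current character index is nonzero.
; When an owner attribute is nonzero, ApplyEffect extends the parent with GE_GenericShieldSteal, deliberately swapping source and target ASCs because it executes only on the target.
; Each steal plays a sound and owner-attached VFX aimed at the victim.
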(event `self.ReceiveBeginPlay`
  (`parent.ReceiveBeginPlay`)
  (`MeshComponent.SetVectorParameterValueOnMaterials` (`self.VisualMesh`) "ColorHit" (`KismetMathLibrary.Conv_LinearColorToVector` (struct :`R` 0.196835 :`G` 0.41873 :`B` 1.0 :`A` 1.0)))
  (`GameplayStatics.PlaySound2D` "/Game/Placeholder/Audio/RPG_Sound_Pack/battle/swing.swing" 1.0 1.0 0.0 null null)
  (bind _asbp_wheel (cast `/Game/Wheel/BP_Wheel` (`self.GetOwner`)))
  (if (not (== (`WheelPawn.CurrentCharacterIndex` _asbp_wheel) 0))
    (bind _output_get (set `self.ShieldSteal` (* (stale _output_get) 0.5)))))

(event `self.OnCharacterHit_Event`
  (params (HitActor :type "Actor Object Reference"))
  (`parent.OnCharacterHit_Event` HitActor))

(event `self.ApplyEffect`
  (params (Actor :type "Actor Object Reference") (TouchedASC :type "AbilitySystemComponent Object Reference"))
  (bind _ownerasc (`self.OwnerASC`))
  (`parent.ApplyEffect` Actor TouchedASC)
  (if (not (== (`.ReturnValue` (`AbilitySystemBlueprintLibrary.GetFloatAttributeFromAbilitySystemComponent` _ownerasc (struct :`AttributeName` "ShieldStealPotency" :`Attribute` "/Script/Curseel.AttributeSetBase:ShieldStealPotency" :`AttributeOwner` "/Script/CoreUObject.Class'\"/Script/Curseel.AttributeSetBase\"'"))) 0.0))
    (`CurseelBlueprintFunctionLibrary.ApplyEffect` (make `GameplayEffectApplier` TouchedASC _ownerasc "Target" "/Game/Blueprints/GE_GenericShieldSteal.GE_GenericShieldSteal_C" (struct :`TagName` "Data.ShieldSteal") (`self.ShieldSteal`)))
    (`GameplayStatics.PlaySound2D` "/Game/Placeholder/Audio/UI_pack_1/ETRA.ETRA" 1.0 1.0 0.0 null null)
    (bind _returnvalue (`NiagaraFunctionLibrary.SpawnSystemAttached` "/Game/Placeholder/VFX_Steal.VFX_Steal" (`Actor.RootComponent` (`self.GetOwner`)) "None" (0.0 0.0 0.0) (struct) "KeepRelativeOffset" true))
    (`NiagaraComponent.SetVariablePosition` _returnvalue "TargetPos" (`self.K2_GetActorLocation` Actor))
    (`NiagaraComponent.SetVariableLinearColor` _returnvalue "Color" (`KismetMathLibrary.LinearColorLerp` (struct :`R` 0.17724 :`G` 0.445348 :`B` 0.895833 :`A` 1.0)))))

(fn `UserConstructionScript`
  (`parent.UserConstructionScript`))