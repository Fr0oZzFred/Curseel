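; Modular dungeon wall builder that lays alternating pillar and wall instances along local Y, with optional pillars at either end.
; The construction script rebuilds both instanced mesh components, spacing them by mesh bounds plus an offset and choosing regular or dissolvable meshes.
; Each actor records its end position and snaps to that of its LinkedWalls actor to form chains, with an event repeating this update.
; ForceSelectionable restores regular meshes and enables distance field lighting.
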(event `Update100_TimesLinkedWalls`
  (for _ (range 101)
    (`self.UpdateLinkedWalls`)))

(event `UpdateLinkedWalls`
  (bind _linkedwalls (`self.LinkedWalls`))
  (set `self.LastPillarWorldPos` (`KismetMathLibrary.TransformLocation` (`self.GetTransform`) (`KismetMathLibrary.MakeVector` 0.0 (* (+ (`self.Count`) 1) (* (+ (`self.GetBoxBoundsY` (`self.GetPillar`)) (`self.GetBoxBoundsY` (`self.GetWall`)) (`self.DistanceOffset`)) 2.0)))))
  (if (and (`KismetSystemLibrary.IsValid` _linkedwalls) (!= _linkedwalls self))
    (`self.K2_SetActorLocation` (`/Game/Dungeon/Walls/BP_Walls.LastPillarWorldPos` _linkedwalls))))

(fn `CreatePattern`
  (params (CurrentDistance :type "Float (double-precision)"))
  (`InstancedStaticMeshComponent.AddInstance` (`self.Pillars`) (`KismetMathLibrary.MakeTransform` (`KismetMathLibrary.MakeVector` 0.0 CurrentDistance)) false)
  (`InstancedStaticMeshComponent.AddInstance` (`self.Walls`) (`KismetMathLibrary.MakeTransform` (`KismetMathLibrary.MakeVector` 0.0 (+ (`self.GetBoxBoundsY` (`self.GetPillar`)) (`self.GetBoxBoundsY` (`self.GetWall`)) (`local.CurrentDistance`) (`self.DistanceOffset`)))) false))

(fn `CreateWalls`
  (`|ExecutionSequence`
    (:`then_0`
      (`InstancedStaticMeshComponent.ClearInstances` (`self.Pillars`))
      (`InstancedStaticMeshComponent.ClearInstances` (`self.Walls`))
      ;[1 1 1] Init Meshes
      (`StaticMeshComponent.SetStaticMesh` (`self.Pillars`) (`self.GetPillar`))
      (`StaticMeshComponent.SetStaticMesh` (`self.Walls`) (`self.GetWall`)))
    (:`then_1`
      (if (`self.bStartWithPillar`)
        (`self.CreatePattern` 0.0)
        (else
          (`InstancedStaticMeshComponent.AddInstance` (`self.Walls`) (`KismetMathLibrary.MakeTransform` (`KismetMathLibrary.MakeVector` 0.0 (+ (`self.GetBoxBoundsY` (`self.GetPillar`)) (`self.GetBoxBoundsY` (`self.GetWall`)) (`self.DistanceOffset`)))) false))))
    (:`then_2`
      (for _index (range 1 (+ (`self.Count`) 1))
        (bind _returnvalue (* _index (* (+ (`self.GetBoxBoundsY` (`self.GetPillar`)) (`self.GetBoxBoundsY` (`self.GetWall`)) (`self.DistanceOffset`)) 2.0)))
        (`self.CreatePattern` _returnvalue))
      (if (`self.bEndWithPillar`)
        (bind _returnvalue_2 (`InstancedStaticMeshComponent.AddInstance` (`self.Pillars`) (`KismetMathLibrary.MakeTransform` (`KismetMathLibrary.MakeVector` 0.0 _returnvalue)) false))
        (set `self.LastPillarWorldPos` (.location (`InstancedStaticMeshComponent.GetInstanceTransform` (`self.Pillars`) _returnvalue_2 true)))))
    (:`then_3`
      (`self.UpdateLinkedWalls`))))

(fn `GetBoxBoundsY`
  (params (StaticMesh :type "StaticMesh Object Reference"))
  (returns (Y :type "Float (double-precision)"))
  (bind (_returnvalue_origin _returnvalue_boxextent) (`KismetMathLibrary.BreakBoxSphereBounds` (`StaticMesh.GetBounds` StaticMesh)))
  (return (.y _returnvalue_boxextent)))

(fn `GetDissolvableMesh`
  (params (DissolvableMesh :type "DissolvableMesh Object Reference"))
  (returns (ReturnValue :type "StaticMesh Object Reference"))
  (return (select `bool` (`self.bDissolvable`) :`false` (`DissolvableMesh.Mesh` DissolvableMesh) :`true` (`DissolvableMesh.DissolvableMesh` DissolvableMesh))))

(fn `GetPillar`
  (returns (Pillar :type "StaticMesh Object Reference"))
  (return (`self.GetDissolvableMesh` (`self.Pillar`))))

(fn `GetWall`
  (returns (Wall :type "StaticMesh Object Reference"))
  (return (`self.GetDissolvableMesh` (`self.Wall`))))

(fn `UserConstructionScript`
  (`self.CreateWalls`)
  (`PrimitiveComponent.SetAffectDistanceFieldLighting` (`self.Walls`) (`self.bAffectDistanceFieldLighting`))
  (`PrimitiveComponent.SetAffectDistanceFieldLighting` (`self.Pillars`) (`self.bAffectDistanceFieldLighting`))
  (if (`self.bForceSelectionable`)
    (`PrimitiveComponent.SetAffectDistanceFieldLighting` (`self.Walls`) true)
    (`PrimitiveComponent.SetAffectDistanceFieldLighting` (`self.Pillars`) true)
    (`StaticMeshComponent.SetStaticMesh` (`self.Pillars`) (`DissolvableMesh.Mesh` (`self.Pillar`)))
    (`StaticMeshComponent.SetStaticMesh` (`self.Walls`) (`DissolvableMesh.Mesh` (`self.Wall`)))))