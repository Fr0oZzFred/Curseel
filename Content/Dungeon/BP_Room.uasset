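; BP_Room is a dungeon room volume that detects when the player enters or leaves it.
; The construction script sets the Box component's extent from the Size variable.
; Box overlaps pass through IsPlayer, which checks the other actor for the "Player" tag, then fire OnPlayerEnter or OnPlayerExit.
; Both events are empty hooks with no room behavior of their own.
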(event `self.Box.OnComponentBeginOverlap`
  (params (OverlappedComponent :type "PrimitiveComponent Object Reference") (OtherActor :type "Actor Object Reference") (OtherComp :type "PrimitiveComponent Object Reference") (OtherBodyIndex :type Integer) (bFromSweep :type Boolean) (SweepResult :type "HitResult Structure (by ref)"))
  (`self.IsPlayer` OtherActor
    (:`true`
      (`self.OnPlayerEnter`))))

(event `self.Box.OnComponentEndOverlap`
  (params (OverlappedComponent :type "PrimitiveComponent Object Reference") (OtherActor :type "Actor Object Reference") (OtherComp :type "PrimitiveComponent Object Reference") (OtherBodyIndex :type Integer))
  (`self.IsPlayer` OtherActor
    (:`true`
      (`self.OnPlayerExit`))))

(event `OnPlayerEnter`)

(event `OnPlayerExit`)

(fn `UserConstructionScript`
  (`BoxComponent.SetBoxExtent` (`self.Box`) (`self.Size`) false))