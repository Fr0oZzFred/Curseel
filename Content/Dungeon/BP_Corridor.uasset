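; Dungeon corridor Blueprint that plays a trap discovery sequence when the player enters.
; On entry, if the sequence reference is valid, it disables the player pawn's input, starts the sequence player and binds to its finished event.
; When playback ends, it re-enables input and clears the reference, so later entries do not replay the sequence.
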(event `self.OnPlayerEnter`
  (bind _sequenceplayer (`LevelSequenceActor.SequencePlayer` (`self.DiscoverTrapSequence`)))
  (`/Engine/EditorBlueprintResources/StandardMacros.IsValid` (`self.DiscoverTrapSequence`)
    (:`Is Valid`
      (`self.DisableInput` (`GameplayStatics.GetPlayerPawn` 0) null)
      (`MovieSceneSequencePlayer.Play` _sequenceplayer)
      (add `MovieSceneSequencePlayer.OnFinished` _sequenceplayer (delegate `OnCristalDiscoverFinished`)))))

(event `OnCristalDiscoverFinished`
  (`self.EnableInput` (`GameplayStatics.GetPlayerPawn` 0) null)
  (set `self.DiscoverTrapSequence` null))

(fn `UserConstructionScript`
  (`parent.UserConstructionScript`))