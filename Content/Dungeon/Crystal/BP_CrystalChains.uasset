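; Spline-driven crystal chain actor that lays chain links along a path, with colored smoke on each link.
; The construction script spaces oriented instanced meshes by mesh bounds and adds a spline mesh with RiverMaterial per segment.
; UpdateColor passes chain color through custom primitive data and zeroes the Erosion parameter.
; BeginPlay spawns tinted smoke systems at the link transforms, which DeactivateSmoke can switch off.
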(event `self.ReceiveBeginPlay`
  (`self.SpawnSmoke`)
  (`self.UpdateColor`))

(event `DeactivateSmoke`
  (for _array_element (`self.SmokeVFXs`)
    (`ActorComponent.Deactivate` _array_element)))

(event `SpawnSmoke`
  (bind _returnvalue (`self.GetTransform`))
  (bind _chainscale (`self.ChainScale`))
  (bind _returnvalue_2 (`KismetMathLibrary.MakeVector` _chainscale _chainscale _chainscale))
  (for _array_element (`self.SmokeVFXs`)
    (`ActorComponent.K2_DestroyComponent` _array_element))
  (`KismetArrayLibrary.Array_Clear` (`self.SmokeVFXs`))
  (for _index (range (+ (`InstancedStaticMeshComponent.GetInstanceCount` (`self.InstancedStaticMesh`)) 1))
    (bind _returnvalue_3 (`self.GetLocationAtIndex` _index))
    (bind (_returnvalue_location _returnvalue_rotation) (`KismetMathLibrary.BreakTransform` (`KismetMathLibrary.MakeTransform` _returnvalue_3 (`KismetMathLibrary.MakeRotFromX` (- (`self.GetLocationAtIndex` (+ _index 1)) _returnvalue_3)) _returnvalue_2)))
    (bind _returnvalue_4 (`NiagaraFunctionLibrary.SpawnSystemAtLocation` (`self.SmokeVFX`) (`KismetMathLibrary.TransformLocation` _returnvalue _returnvalue_location) (`KismetMathLibrary.TransformRotation` _returnvalue _returnvalue_rotation) _returnvalue_2))
    (`NiagaraComponent.SetVariableLinearColor` _returnvalue_4 "Color" (`self.SmokeColor`))
    (`KismetArrayLibrary.Array_Add` (`self.SmokeVFXs`) _returnvalue_4)))

(fn `GetLocationAtIndex`
  (params (A :type Integer))
  (returns (ReturnValue :type "Vector Structure"))
  (return (`SplineComponent.GetLocationAtDistanceAlongSpline` (`self.Spline`) (* A (`self.Spacing`)) "Local")))

(fn `UpdateColor`
  (bind (_r _g _b _a) (break `LinearColor` (`self.ChainColor`)))
  (`PrimitiveComponent.SetCustomPrimitiveDataVector4` (`self.InstancedStaticMesh`) 0 (`KismetMathLibrary.MakeVector4` _r _g _b _a))
  (`MeshComponent.SetScalarParameterValueOnMaterials` (`self.InstancedStaticMesh`) "Erosion" 0.0))

(fn `UserConstructionScript`
  (locals (InstancesNo :type Integer :default 0))
  (bind (_returnvalue_x _returnvalue_y) (`KismetMathLibrary.BreakVector` (`self.GetActorScale3D`)))
  (bind _spline (`self.Spline`))
  (bind _riverwidth (`self.RiverWidth`))
  (bind _spline_2 (`self.Spline`))
  (bind _riverwidth_2 (`self.RiverWidth`))
  (bind _chainscale (`self.ChainScale`))
  (bind (_min _max) (break `Box` (`StaticMesh.GetBoundingBox` (`self.ChainMesh`))))
  (`|ExecutionSequence`
    (:`then_0`
      (`StaticMeshComponent.SetStaticMesh` (`self.InstancedStaticMesh`) (`self.ChainMesh`))
      (bind _output_get (set `self.Spacing` (+ (.y (- _max _min)) (`self.Offset`))))
      (set `self.Spacing` (* _returnvalue_y (`self.Spacing`)))
      (bind _output_get_2 (set `local.InstancesNo` (`KismetMathLibrary.FFloor` (/ (`SplineComponent.GetSplineLength` (`self.Spline`)) _output_get))))
      (for _index (range (+ _output_get_2 1))
        (bind _returnvalue (`self.GetLocationAtIndex` _index))
        (`InstancedStaticMeshComponent.AddInstance` (`self.InstancedStaticMesh`) (`KismetMathLibrary.MakeTransform` _returnvalue (`KismetMathLibrary.MakeRotFromX` (- (`self.GetLocationAtIndex` (+ _index 1)) _returnvalue)) (`KismetMathLibrary.MakeVector` _chainscale _chainscale _chainscale)) false)))
    (:`then_1`
      (`self.UpdateColor`))
    (:`then_2`
      ;[1 1 1] Comment
      (for _index_2 (range (+ (- (`SplineComponent.GetNumberOfSplinePoints` (`self.Spline`)) 2) 1))
        (bind _returnvalue_2 (`AddComponent|NODE_AddSplineMeshComponent-6`))
        (`PrimitiveComponent.SetMaterial` _returnvalue_2 0 (`self.RiverMaterial`))
        (`StaticMeshComponent.SetStaticMesh` _returnvalue_2 "/Game/Dungeon/Crystal/ChainsSpline.ChainsSpline")
        (bind (_returnvalue_x_2 _returnvalue_y_2) (`KismetMathLibrary.BreakVector` (`SplineComponent.GetScaleAtSplinePoint` _spline_2 _index_2)))
        (`SplineMeshComponent.SetStartScale` _returnvalue_2 (`KismetMathLibrary.MakeVector2D` (* _returnvalue_x_2 _riverwidth) (* _riverwidth _returnvalue_y_2)) true)
        (bind (_returnvalue_x_3 _returnvalue_y_3) (`KismetMathLibrary.BreakVector` (`SplineComponent.GetScaleAtSplinePoint` _spline_2 (+ _index_2 1))))
        (`SplineMeshComponent.SetEndScale` _returnvalue_2 (`KismetMathLibrary.MakeVector2D` (* _returnvalue_x_3 _riverwidth_2) (* _riverwidth_2 _returnvalue_y_3)) true)
        (`SceneComponent.K2_AttachToComponent` _returnvalue_2 null "None" "KeepRelative" "KeepRelative" "KeepRelative" true)
        (bind (_location _tangent) (`SplineComponent.GetLocationAndTangentAtSplinePoint` _spline _index_2 "Local"))
        (bind (_location_2 _tangent_2) (`SplineComponent.GetLocationAndTangentAtSplinePoint` _spline (+ _index_2 1) "Local"))
        (`SplineMeshComponent.SetStartAndEnd` _returnvalue_2 _location _tangent _location_2 _tangent_2 true)))))