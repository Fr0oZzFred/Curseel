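; BP_Symbol is a dungeon symbol that, when activated, damages or heals characters standing in its box, depending on its Damage flag.
; Material scalar parameters on the plane show the chosen state and a timeline-driven Boost ramp during activation.
; When the timeline ends, it applies the matching Gameplay Effect to overlapping actors with a Curseel ASC, fires red or green Niagara VFX and clears its highlight.
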(event `SetChosen`
  (params (Chosen :type Boolean))
  (`MeshComponent.SetScalarParameterValueOnMaterials` (`self.Plane`) "Chosen" (select `bool` Chosen :`true` 1.0 :!type "Float (single-precision)")))

(event `Activate`
  (bind (_direction _alpha) (`Timeline|Timeline` :!via `PlayFromStart`)
    (:`Update`
      (`MeshComponent.SetScalarParameterValueOnMaterials` (`self.Plane`) "Boost" (`KismetMathLibrary.Lerp` 1.0 10.0 _alpha)))
    (:`Finished`
      (`self.CheckForCharacterCollision`)
      (`NiagaraComponent.SetVariableLinearColor` (`self.VFX_Symbol`) "Color" (select `bool` (`self.Damage`) :`false` (make `LinearColor` 0.0 1.0 0.0 1.0) :`true` (make `LinearColor` 1.0 0.0 0.0 1.0) :!type "LinearColor Structure"))
      (`ActorComponent.Activate` (`self.VFX_Symbol`) true)
      (`MeshComponent.SetScalarParameterValueOnMaterials` (`self.Plane`) "Boost" 1.0)
      (`self.SetChosen` false))))

(event `CheckForCharacterCollision`
  (for _array_element (`PrimitiveComponent.GetOverlappingActors` (`self.Box`) null)
    (bind _returnvalue (`CurseelBlueprintFunctionLibrary.GetCurseelASC` _array_element))
    (`/Engine/EditorBlueprintResources/StandardMacros.IsValid` _returnvalue
      (:`Is Valid`
        (`CurseelBlueprintFunctionLibrary.ApplyEffect` (select `bool` (`self.Damage`) :`false` (make `GameplayEffectApplier` _returnvalue null "Source" "/Game/Dungeon/GE_SymbolHeal.GE_SymbolHeal_C") :`true` (make `GameplayEffectApplier` _returnvalue null "Source" "/Game/Dungeon/GE_SymbolDamage.GE_SymbolDamage_C")))))))

(fn `UserConstructionScript`)