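; Dungeon room controller that links a Sigil, a Door and an optional trap actor into one encounter.
; The door opens at start, closes when the sigil activates and reopens when it finishes.
; Traps implementing BPI_RoomTrap are initialized, then activated and deactivated with the sigil.
; On finish a sequence plays while the player has input disabled and a GAS invincibility effect, whose removal follows shortly after input returns.
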(event `SnapPosToSigil`
  (bind _sigil (`self.Sigil`))
  (`/Engine/EditorBlueprintResources/StandardMacros.IsValid` _sigil
    (:`Is Valid`
      (`self.K2_SetActorLocation` (`self.K2_GetActorLocation` _sigil)))))

(event `InitTrapEditor`
  (bind _trapactor (`self.TrapActor`))
  (`/Engine/EditorBlueprintResources/StandardMacros.IsValid` _trapactor
    (:`Is Valid`
      (message `/Game/Dungeon/Traps/BPI_RoomTrap.InitTrap` _trapactor self))))

(event `OnSigilActivated`
  (params (Sigil :type "/Game/Dungeon/Sigil/BP_Sigil Object Reference"))
  (`/Game/Dungeon/Door/BP_DoorBarrier.Close` (`self.Door`)))

(event `self.ReceiveBeginPlay`
  (bind _sigil (`self.Sigil`))
  (`/Game/Dungeon/Door/BP_DoorBarrier.Open` (`self.Door`))
  (`|ExecutionSequence`
    (:`then_0`
      (add `/Game/Dungeon/Sigil/BP_Sigil.OnActivated` (`self.Sigil`) (delegate `OnSigilActivated`)))
    (:`then_1`
      (add `/Game/Dungeon/Sigil/BP_Sigil.OnFinish` (`self.Sigil`) (delegate `OnSigilFinsihed`)))
    (:`then_2`
      (if (`KismetSystemLibrary.DoesImplementInterface` (`self.TrapActor`) "/Game/Dungeon/Traps/BPI_RoomTrap.BPI_RoomTrap_C")
        (message `/Game/Dungeon/Traps/BPI_RoomTrap.InitTrap` (`self.TrapActor`) self)
        (add `/Game/Dungeon/Sigil/BP_Sigil.OnActivated` _sigil (delegate `OnActivated_Event`))
        (add `/Game/Dungeon/Sigil/BP_Sigil.OnFinish` _sigil (delegate `OnDeactivate`))
        (else
          (`KismetSystemLibrary.PrintString` (`KismetStringLibrary.Concat_StrStr` (`KismetSystemLibrary.GetDisplayName` (`self.TrapActor`)) "is not a trap")))))))

(event `OnSigilFinsihed`
  (params (Sigil :type "/Game/Dungeon/Sigil/BP_Sigil Object Reference"))
  (bind _returnvalue (`AbilitySystemBlueprintLibrary.GetAbilitySystemComponent` (`GameplayStatics.GetPlayerPawn` 0)))
  (bind _sequenceplayer (`LevelSequenceActor.SequencePlayer` (`self.SequenceOnFinish`)))
  (`/Game/Dungeon/Door/BP_DoorBarrier.Open` (`self.Door`))
  (`self.DisableInput` (`GameplayStatics.GetPlayerPawn` 0) null)
  (`MovieSceneSequencePlayer.Play` _sequenceplayer)
  (add `MovieSceneSequencePlayer.OnFinished` _sequenceplayer (delegate `OnSequenceFinish`))
  (`AbilitySystemComponent.BP_ApplyGameplayEffectSpecToSelf` _returnvalue (`AbilitySystemComponent.MakeOutgoingSpec` :`self` _returnvalue :`GameplayEffectClass` "/Game/Blueprints/GE_Invincible.GE_Invincible_C")))

(event `OnSequenceFinish`
  (`self.EnableInput` (`GameplayStatics.GetPlayerPawn` 0) null)
  (`KismetSystemLibrary.Delay` 1.0)
  (`AbilitySystemComponent.RemoveActiveEffectsWithTags` (`AbilitySystemBlueprintLibrary.GetAbilitySystemComponent` (`GameplayStatics.GetPlayerPawn` 0)) (struct :`GameplayTags` (struct :`(TagName` "State.Buff.Invicible")))))

(event `OnActivated_Event`
  (params (Sigil :type "/Game/Dungeon/Sigil/BP_Sigil Object Reference"))
  (message `/Game/Dungeon/Traps/BPI_RoomTrap.Activate` (`self.TrapActor`)))

(event `OnDeactivate`
  (params (Sigil :type "/Game/Dungeon/Sigil/BP_Sigil Object Reference"))
  (message `/Game/Dungeon/Traps/BPI_RoomTrap.Deactivate` (`self.TrapActor`)))

(fn `BindOnSequenceFinished`
  (params (Event :type "Delegate (by ref)"))
  (add `MovieSceneSequencePlayer.OnFinished` (`LevelSequenceActor.SequencePlayer` (`self.SequenceOnFinish`)) Event))

(fn `UserConstructionScript`
  (`parent.UserConstructionScript`))