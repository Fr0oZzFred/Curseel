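; Sigil actor for a round-based monster challenge, activated by interacting while the player is inside its radius.
; Activation starts three looping timers that spawn chasing wolves around world origin, throttled by a live-monster cap.
; Monster deaths inside the radius fill the VFX progress; completion stops spawning and destroys remaining monsters.
; Interacting again opens the boost menu; choosing a boost replaces the sigil with a next-round copy.
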(event `self.ReceiveBeginPlay`
  (bind _asbp_wheel (cast `/Game/Blueprints/Bp_Wheel` (`GameplayStatics.GetPlayerPawn` 0)))
  (bind _output_get (set `self.PlayerWheel` _asbp_wheel))
  (add `/Game/Blueprints/Bp_Wheel.OnInteract` _output_get (delegate `OnInteract_Event`))
  (add `self.OnPlayerEnterSigil` (delegate `OnPlayerEnterSigil_Event`))
  (add `self.OnPlayerLeaveSigil` (delegate `OnPlayerLeaveSigil_Event`)))

(event `OnPlayerEnterSigil_Event`
  (if (or (not (`self.Activated`)) (`self.Done`))
    (`FXSystemComponent.SetColorParameter` (`self.VFX_Sigil`) "Color" (struct :`R` 1.0 :`G` 1.0 :`B` 1.0 :`A` 1.0))
    (`SceneComponent.SetVisibility` (`self.Interact`) true false)))

(event `OnPlayerLeaveSigil_Event`
  (if (or (not (`self.Activated`)) (`self.Done`))
    (`FXSystemComponent.SetColorParameter` (`self.VFX_Sigil`) "Color" (struct :`A` 1.0))
    (`SceneComponent.SetVisibility` (`self.Interact`) false false)))

(event `OnInteract_Event`
  (bind _playerwheel (`self.PlayerWheel`))
  (if (`self.Done`)
    (`EnhancedInputSubsystemInterface.ClearAllMappings` (pcsubsystem `EnhancedInputLocalPlayerSubsystem` (cast `PlayerController` (`Pawn.GetController` _playerwheel) :!pure true)))
    (bind _pushedwidget (`/Game/UI/W_Overall_UI_Layout.PushWidgetToLayerStack` (`/Game/GameModes/InGame/HUD_InGame.Overall_UI_Layout` (`/Game/Blueprints/Bp_Wheel.HUD_InGame` _playerwheel)) (struct :`TagName` "UI.Layer.GameMenu") "/Game/UI/W_BoostMenu.W_BoostMenu_C"))
    (bind _asw_boost_menu (cast `/Game/UI/W_BoostMenu` _pushedwidget))
    (add `/Game/UI/W_BoostMenu.OnBoostChose` _asw_boost_menu (delegate `OnBoostChose_Event`))
    (elif (and (`self.PlayerIsInRange`) (not (`self.Activated`)))
      (set `self.Activated` true)
      (`SceneComponent.SetVisibility` (`self.Interact`) false false)
      (`FXSystemComponent.SetColorParameter` (`self.VFX_Sigil`) "Color" (struct :`A` 1.0))
      (`self.SetActorTickEnabled` false)
      (`self.SpawnMonsters`))))

(event `OnBoostChose_Event`
  (bind _returnvalue (pcsubsystem `EnhancedInputLocalPlayerSubsystem` (cast `PlayerController` (`Pawn.GetController` (`self.PlayerWheel`)) :!pure true)))
  (`EnhancedInputSubsystemInterface.AddMappingContext` _returnvalue "/Game/Inputs/IMC_SystemInGame.IMC_SystemInGame" 0 (struct))
  (`EnhancedInputSubsystemInterface.AddMappingContext` _returnvalue "/Game/Inputs/IMC_WheelDefault.IMC_WheelDefault" 0 (struct))
  (`self.OnFinish`)
  (remove `/Game/Blueprints/Bp_Wheel.OnInteract` (stale `self.ReceiveBeginPlay` _output_get) (delegate `OnInteract_Event`))
  (`SceneComponent.SetVisibility` (`self.Interact`) false false)
  (`self.SetActorTickEnabled` false)
  (`|SpawnActorFromClass` "BP_Sigil_V2_C" (`self.GetTransform`) "Undefined" "MultiplyWithRoot" null (+ (`self.Round`) 1) null)
  (`self.K2_DestroyActor`))

(event `self.ReceiveTick`
  (params (DeltaSeconds :type "Float (single-precision)"))
  (if (< (`KismetMathLibrary.Abs` (`KismetMathLibrary.Vector_Distance` (`self.K2_GetActorLocation` (`self.PlayerWheel`)) (`self.K2_GetActorLocation`))) (`self.Radius`))
    (if (not (`self.PlayerIsInRange`))
      (set `self.PlayerIsInRange` true)
      (`self.OnPlayerEnterSigil`))
    (elif (`self.PlayerIsInRange`)
      (set `self.PlayerIsInRange` false)
      (`self.OnPlayerLeaveSigil`))))

(event `SpawnMonsters`
  (bind _returnvalue (`KismetSystemLibrary.K2_SetTimerDelegate` (delegate `CustomEvent`) 5.0 true 0.0 2.0))
  (bind _returnvalue_2 (`KismetSystemLibrary.K2_SetTimerDelegate` (delegate `CustomEvent`) 4.0 true 0.0 1.0))
  (bind _returnvalue_3 (`KismetSystemLibrary.K2_SetTimerDelegate` (delegate `CustomEvent`) 3.0 true 0.0 1.0)))

(event `CustomEvent`
  (bind _returnvalue (* (`KismetMathLibrary.RandomFloatInRange` 0.0 1.0) (`KismetMathLibrary.GetTAU`)))
  (bind _result (`/Engine/EditorBlueprintResources/StandardMacros.IncrementInt` (`self.SpawnCount`))
    (:`  `
      (if (< (`self.MonstersCount`) 20)
        (for _ (range (+ (`KismetMathLibrary.Clamp` _result 0 2) 1))
          (`/Engine/EditorBlueprintResources/StandardMacros.IncrementInt` (`self.MonstersCount`)
            (:`  `
              (bind _returnvalue_2 (`|SpawnActorFromClass` (`KismetArrayLibrary.Array_Random` (`|MakeArray` "/Game/Monsters/BP_Wolf.BP_Wolf_C" :!type "Actor Class Reference")) (`KismetMathLibrary.MakeTransform` (+ (0.0 0.0 0.0) (`KismetMathLibrary.MakeVector` (* (`KismetMathLibrary.Cos` _returnvalue) 1000.0) (* (`KismetMathLibrary.Sin` _returnvalue) 1000.0)))) "Undefined" "MultiplyWithRoot" null null))
              (bind _asbp_monster_character (cast `/Game/Monsters/BP_MonsterCharacter` _returnvalue_2))
              (`/Game/Monsters/BP_MonsterCharacter.ChasePlayer` _asbp_monster_character)
              (add `self.OnDestroyed` _asbp_monster_character (delegate `OnDestroyed_Event`)))))))))

(event `OnDestroyed_Event` :!signature `self.OnDestroyed`
  (params (DestroyedActor :type "Actor Object Reference"))
  (bind _monsterskilled (`self.MonstersKilled`))
  (bind _returnvalue (/ (`KismetMathLibrary.Conv_IntToDouble` _monsterskilled) (`KismetMathLibrary.Conv_IntToDouble` (`self.MonsterRequirement`))))
  (`/Engine/EditorBlueprintResources/StandardMacros.DecrementInt` (`self.MonstersCount`)
    (:`  `
      (if (< (`KismetMathLibrary.Vector_Distance` (`self.K2_GetActorLocation` DestroyedActor) (`self.K2_GetActorLocation`)) (`self.Radius`))
        (`/Engine/EditorBlueprintResources/StandardMacros.IncrementInt` _monsterskilled
          (:`  `
            (`FXSystemComponent.SetFloatParameter` (`self.VFX_Sigil`) "Progression" _returnvalue)
            (bind _output_get (set `self.Done` (>= _returnvalue 1.0)))
            (if _output_get
              (`NiagaraFunctionLibrary.SpawnSystemAttached` "/Game/Placeholder/VFX_SigilWin.VFX_SigilWin" (`self.VFX_Sigil`) "None" (0.0 0.0 0.0) (struct) "KeepRelativeOffset")
              (`KismetSystemLibrary.K2_ClearAndInvalidateTimerHandle` (stale `SpawnMonsters` _returnvalue))
              (`KismetSystemLibrary.K2_ClearAndInvalidateTimerHandle` (stale `SpawnMonsters` _returnvalue_2))
              (`KismetSystemLibrary.K2_ClearAndInvalidateTimerHandle` (stale `SpawnMonsters` _returnvalue_3))
              (bind _outactors (`GameplayStatics.GetAllActorsOfClass` "/Game/Monsters/BP_MonsterCharacter.BP_MonsterCharacter_C"))
              (for _array_element _outactors
                (`self.K2_DestroyActor` _array_element))
              (bind _asw_interact_3d (cast `/Game/UI/W_Interact3D` (`WidgetComponent.GetWidget` (`self.Interact`))))
              (`/Game/UI/W_Interact3D.SetTextToClaim` _asw_interact_3d)
              (`SceneComponent.SetVisibility` (`self.Interact`) true false)
              (`self.SetActorTickEnabled` true)
              (bind _asw_game (cast `/Game/UI/W_Game` (`/Game/GameModes/InGame/HUD_InGame.W_Game` (`/Game/Blueprints/Bp_Wheel.HUD_InGame` (`self.PlayerWheel`)))))
              (`/Game/UI/W_Game.DisplayMessage` _asw_game (`|FormatText` "Round {round} done !" (`self.Round`))))))))))

(fn `UserConstructionScript`
  (`FXSystemComponent.SetFloatParameter` (`self.VFX_Sigil`) "Radius" (* (`self.Radius`) 2.0)))