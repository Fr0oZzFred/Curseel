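; BP_Sigil is a dungeon wave trigger that the player activates by interacting within its radius to start a round of monsters.
; A Tick distance check toggles the prompt and VFX highlight, and pauses during the fight.
; Monsters spawn from the DTPattern data table, and their OnDestroyed events drive the Niagara progression until the round is done.
; Interacting again then respawns the sigil with the next round number, shows a message and destroys itself.
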(event `self.ReceiveBeginPlay`
  (bind _asbp_wheel_character (cast `/Game/MainCharacters/BP_WheelCharacter` (`GameplayStatics.GetPlayerPawn` 0)))
  (bind _output_get (set `self.WheelCharacter` _asbp_wheel_character))
  (add `/Game/MainCharacters/BP_WheelCharacter.OnInteract` _output_get (delegate `OnInteract_Event_0`))
  (add `self.OnPlayerEnterSigil` (delegate `OnPlayerEnterSigil_Event`))
  (add `self.OnPlayerLeaveSigil` (delegate `OnPlayerLeaveSigil_Event`)))

(event `OnInteract_Event_0`
  (if (`self.Done`)
    (`|SpawnActorFromClass` "BP_Sigil_C" (`self.GetTransform`) "Undefined" "MultiplyWithRoot" null (+ (`self.Round`) 1) null)
    (bind _asw_game (cast `/Game/UI/W_Game` (`/Game/GameModes/InGame/HUD_InGame.W_Game` (`/Game/GameModes/InGame/GM_InGame.HUD` (cast `/Game/GameModes/InGame/GM_InGame` (`GameplayStatics.GetGameMode`) :!pure true)))))
    (`/Game/UI/W_Game.DisplayMessage` _asw_game (`|FormatText` "Round {round} done !" (`self.Round`)))
    (`self.K2_DestroyActor`)
    (elif (and (`self.PlayerIsInRange`) (not (`self.Activated`)))
      (set `self.Activated` true)
      (`SceneComponent.SetVisibility` (`self.Interact`) false false)
      (`FXSystemComponent.SetColorParameter` (`self.VFX_Sigil`) "Color" (struct :`A` 1.0))
      (`self.SetActorTickEnabled` false)
      (`self.SpawnMonsters`))))

(event `OnPlayerEnterSigil_Event`
  (if (or (not (`self.Activated`)) (`self.Done`))
    (`FXSystemComponent.SetColorParameter` (`self.VFX_Sigil`) "Color" (struct :`R` 1.0 :`G` 1.0 :`B` 1.0 :`A` 1.0))
    (`SceneComponent.SetVisibility` (`self.Interact`) true false)))

(event `OnPlayerLeaveSigil_Event`
  (if (or (not (`self.Activated`)) (`self.Done`))
    (`FXSystemComponent.SetColorParameter` (`self.VFX_Sigil`) "Color" (struct :`A` 1.0))
    (`SceneComponent.SetVisibility` (`self.Interact`) false false)))

(event `self.ReceiveTick`
  (params (DeltaSeconds :type "Float (single-precision)"))
  (if (< (`KismetMathLibrary.Abs` (`KismetMathLibrary.Vector_Distance` (`self.K2_GetActorLocation` (`self.WheelCharacter`)) (`self.K2_GetActorLocation`))) (`self.Radius`))
    (if (not (`self.PlayerIsInRange`))
      (set `self.PlayerIsInRange` true)
      (`self.OnPlayerEnterSigil`))
    (elif (`self.PlayerIsInRange`)
      (set `self.PlayerIsInRange` false)
      (`self.OnPlayerLeaveSigil`))))

(event `SpawnMonsters`
  (bind _dt_pattern (`self.DT_Pattern`))
  (`KismetSystemLibrary.K2_SetTimerDelegate` (delegate `CheckSpawn`) 0.5 true)
  (bind _outrownames (`DataTableFunctionLibrary.GetDataTableRowNames` _dt_pattern))
  (set `self.MonstersCount` (`KismetArrayLibrary.Array_Length` _outrownames))
  (for _array_element _outrownames
    (bind _returnvalue (`|GetDataTableRow` _dt_pattern _array_element)
      (:`then`
        (bind (_monster _location) (break `/Game/Dungeon/Sigil/S_MonstersSpawn` _returnvalue))
        (bind _returnvalue_2 (`|SpawnActorFromClass` _monster (`KismetMathLibrary.MakeTransform` (`KismetMathLibrary.InverseTransformLocation` (`self.GetTransform`) (select `bool` (`self.RandomPos`) :`false` _location :`true` (* (`KismetMathLibrary.RandomUnitVector`) (1000.0 1000.0 0.0))))) "Undefined" "MultiplyWithRoot" null null))
        (add `self.OnDestroyed` _returnvalue_2 (delegate `OnDestroyed_Event`))))))

(event `OnDestroyed_Event` :!signature `self.OnDestroyed`
  (params (DestroyedActor :type "Actor Object Reference"))
  (bind _monsterskilled (`self.MonstersKilled`))
  (bind _returnvalue (/ (`KismetMathLibrary.Conv_IntToDouble` _monsterskilled) (`KismetMathLibrary.Conv_IntToDouble` (`self.MonstersCount`))))
  (`/Engine/EditorBlueprintResources/StandardMacros.IncrementInt` _monsterskilled
    (:`  `
      (`FXSystemComponent.SetFloatParameter` (`self.VFX_Sigil`) "Progression" _returnvalue)
      (bind _output_get (set `self.Done` (>= _returnvalue 1.0)))
      (if _output_get
        (`NiagaraFunctionLibrary.SpawnSystemAttached` "/Game/Placeholder/VFX_SigilWin.VFX_SigilWin" (`self.VFX_Sigil`) "None" (0.0 0.0 0.0) (struct) "KeepRelativeOffset")
        (bind _asw_interact_3d (cast `/Game/UI/W_Interact3D` (`WidgetComponent.GetWidget` (`self.Interact`))))
        (`/Game/UI/W_Interact3D.SetTextToClaim` _asw_interact_3d)
        (`self.SetActorTickEnabled` true)))))

(event `CheckSpawn`
  (bind _output_get (set `self.CurTimer` (+ (stale _output_get) 0.5))))

(fn `UserConstructionScript`
  (`FXSystemComponent.SetFloatParameter` (`self.VFX_Sigil`) "Radius" (* (`self.Radius`) 2.0)))