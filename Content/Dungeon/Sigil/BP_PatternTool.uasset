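; BP_PatternTool is a Sigil helper actor that visualizes a Pattern data table as capsule components.
; Construction and the Refresh event both call NewFunction, which destroys the previous capsules and rebuilds one per table row.
; Each capsule sits at the row's Location, raised by a fixed height and scaled up, with collision disabled and visibility in game enabled.
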(event `Refresh`
  (`self.NewFunction`))

(fn `NewFunction`
  (bind _pattern (`self.Pattern`))
  (bind _capsulecomponents (`self.CapsuleComponents`))
  (for _array_element _capsulecomponents
    (`ActorComponent.K2_DestroyComponent` _array_element))
  (`KismetArrayLibrary.Array_Clear` _capsulecomponents)
  (`/Engine/EditorBlueprintResources/StandardMacros.IsValid` _pattern
    (:`Is Valid`
      (bind _outrownames (`DataTableFunctionLibrary.GetDataTableRowNames` _pattern))
      (for _array_element_2 _outrownames
        (bind _returnvalue (`|GetDataTableRow` (`self.Pattern`) _array_element_2)
          (:`then`
            (bind _returnvalue_2 (`AddComponent|NODE_AddCapsuleComponent-0` :`RelativeTransform` (`KismetMathLibrary.MakeTransform` (+ (`.Location_7_3F88DFC94856C342043E18A5F2CEC39D` (break `/Game/Dungeon/Sigil/S_MonstersSpawn` _returnvalue)) (0.0 0.0 89.0)) (struct) (2.0 2.0 2.0))))
            (`KismetArrayLibrary.Array_Add` (`self.CapsuleComponents`) _returnvalue_2)
            (`PrimitiveComponent.SetCollisionEnabled` _returnvalue_2 "NoCollision")
            (`SceneComponent.SetHiddenInGame` _returnvalue_2 false false)))))))

(fn `UserConstructionScript`
  (`self.NewFunction`))