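; BP_FirstRoom is the dungeon's first-room controller, tying two doors to the progress of a Sigil.
; On BeginPlay it opens FirstDoor, closes DoorToCristal and binds to the Sigil's activated and finish events.
; Sigil activation shuts FirstDoor, and its completion opens DoorToCristal.
; A separate SnapPosToSigil event moves the actor to the Sigil's location when that reference is valid.
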(event `SnapPosToSigil`
  (bind _sigil (`self.Sigil`))
  (`/Engine/EditorBlueprintResources/StandardMacros.IsValid` _sigil
    (:`Is Valid`
      (`self.K2_SetActorLocation` (`self.K2_GetActorLocation` _sigil)))))

(event `self.ReceiveBeginPlay`
  (bind _sigil (`self.Sigil`))
  (`/Game/Dungeon/Door/BP_DoorBarrier.Open` (`self.FirstDoor`))
  (`/Game/Dungeon/Door/BP_DoorBarrier.Close` (`self.DoorToCristal`))
  (`|ExecutionSequence`
    (:`then_0`
      (add `/Game/Dungeon/Sigil/BP_Sigil.OnActivated` _sigil (delegate `OnSigilActivated`)))
    (:`then_1`
      (add `/Game/Dungeon/Sigil/BP_Sigil.OnFinish` _sigil (delegate `OnSigilFinsihed`)))))

(event `OnSigilActivated`
  (params (Sigil :type "/Game/Dungeon/Sigil/BP_Sigil Object Reference"))
  (`/Game/Dungeon/Door/BP_DoorBarrier.Close` (`self.FirstDoor`)))

(event `OnSigilFinsihed`
  (params (Sigil :type "/Game/Dungeon/Sigil/BP_Sigil Object Reference"))
  (`/Game/Dungeon/Door/BP_DoorBarrier.Open` (`self.DoorToCristal`)))

(fn `UserConstructionScript`
  (`parent.UserConstructionScript`))