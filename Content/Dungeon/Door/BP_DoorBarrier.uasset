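; BP_DoorBarrier is a dungeon door barrier that blocks passage with a visual effect and collision.
; Open deactivates and hides the barrier effect and disables the actor's collision, while Close activates it, shows it and enables collision.
; On BeginPlay it calls one of these according to the StartOpen flag.
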(event `self.ReceiveBeginPlay`
  (if (`self.StartOpen`)
    (`self.Open`)
    (else
      (`self.Close`))))

(event `Open`
  (`ActorComponent.Deactivate` (`self.VFX_DoorBarrier`))
  (`SceneComponent.SetVisibility` (`self.VFX_DoorBarrier`) false false)
  (`self.SetActorEnableCollision` false))

(event `Close`
  (`ActorComponent.Activate` (`self.VFX_DoorBarrier`) true)
  (`SceneComponent.SetVisibility` (`self.VFX_DoorBarrier`) true false)
  (`self.SetActorEnableCollision` true))

(fn `UserConstructionScript`)