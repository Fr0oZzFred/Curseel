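; BP_CristalRoom is the dungeon's crystal room, serving as the discovery moment and later the gateway to the boss level.
; First player entry plays a one-time discovery sequence with dialogue, disabling input until it finishes.
; PrepareForFinalPhase skips that intro, spawns VFX, arms the crystal's overlap box, and queues end-of-progression dialogue after the sigil room's sequence.
; A BP_Wheel entering the box saves its active boosts to the GameInstance, then opens Boss.
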(event `self.OnPlayerEnter`
  (bind _sequenceplayer (`LevelSequenceActor.SequencePlayer` (`self.DiscoverCristalSequence`)))
  (`parent.OnPlayerEnter`)
  (`/Engine/EditorBlueprintResources/StandardMacros.IsValid` (`self.DiscoverCristalSequence`)
    (:`Is Valid`
      (`self.DisableInput` (`GameplayStatics.GetPlayerPawn` 0) null)
      (`MovieSceneSequencePlayer.Play` _sequenceplayer)
      (add `MovieSceneSequencePlayer.OnFinished` _sequenceplayer (delegate `OnCristalDiscoverFinished`))
      (`/Game/Dialogues/BP_DialogueManager.TryToStartDialogue` (`/Game/GameModes/InGame/GM_InGame.DialogueManager` (cast `/Game/GameModes/InGame/GM_InGame` (`GameplayStatics.GetGameMode`) :!pure true)) "/Game/Dialogues/DT_CristalDiscoveryDialogue.DT_CristalDiscoveryDialogue"))))

(event `OnCristalDiscoverFinished`
  (`self.EnableInput` (`GameplayStatics.GetPlayerPawn` 0) null)
  (set `self.DiscoverCristalSequence` null))

(event `PrepareForFinalPhase`
  (params (Sigil :type "/Game/Dungeon/Sigil/BP_Sigil Object Reference"))
  (set `self.DiscoverCristalSequence` null) ; For faster editor test
  (`/Game/Dungeon/BP_SigilRoom.BindOnSequenceFinished` (cast `/Game/Dungeon/BP_SigilRoom` (`/Game/Dungeon/Sigil/BP_Sigil.Room` Sigil) :!pure true) (delegate `OnSigilSequenceFinished`))
  (add `PrimitiveComponent.OnComponentBeginOverlap` (`self.CrystalInteractBox`) (delegate `OnComponentBeginOverlap_Event`))
  (`NiagaraFunctionLibrary.SpawnSystemAtLocation` "/Game/Placeholder/VFX_Spawn1.VFX_Spawn1" (`KismetMathLibrary.TransformLocation` (`self.GetTransform`) (0.0 0.0 1.0))))

(event `OnSigilSequenceFinished`
  (`/Game/Dialogues/BP_DialogueManager.TryToStartDialogue` (`/Game/GameModes/InGame/GM_InGame.DialogueManager` (cast `/Game/GameModes/InGame/GM_InGame` (`GameplayStatics.GetGameMode`) :!pure true)) "/Game/Dialogues/DT_OnProgEnd.DT_OnProgEnd"))

(event `OnComponentBeginOverlap_Event`
  (params (OverlappedComponent :type "PrimitiveComponent Object Reference") (OtherActor :type "Actor Object Reference") (OtherComp :type "PrimitiveComponent Object Reference") (OtherBodyIndex :type Integer) (bFromSweep :type Boolean) (SweepResult :type "HitResult Structure (by ref)"))
  (bind _asbp_wheel (cast `/Game/Wheel/BP_Wheel` OtherActor))
  (set `/Game/Blueprints/GI_Curseel.CurrentBoosts` (`PawnBase.ActiveBoosts` _asbp_wheel) (cast `/Game/Blueprints/GI_Curseel` (`GameplayStatics.GetGameInstance`) :!pure true))
  (`GameplayStatics.OpenLevelBySoftObjectPtr` "/Game/Levels/Boss.Boss"))

(fn `UserConstructionScript`
  (`parent.UserConstructionScript`)
  (`BoxComponent.SetBoxExtent` (`self.CrystalInteractBox`) (`self.CrystalBox`) false))