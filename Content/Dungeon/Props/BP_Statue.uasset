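; BP_Statue is a dungeon statue prop that the player can interact with or hit with a matching character AOE.
; When interactable and in range, the player's wheel interact plays a level sequence with input disabled, then fires OnInteracted.
; While its VFX is visible, overlaps from the filtered Benelu, Kyana or Tolg AOE fire OnAttacked with hit effects and sound.
; The construction script snaps the linked sequence actor to the statue.
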(event `self.ReceiveBeginPlay`
  (bind _asbp_wheel (cast `/Game/Wheel/BP_Wheel` (`GameplayStatics.GetPlayerPawn` 0)))
  (add `WheelPawn.OnInteract` _asbp_wheel (delegate `OnInteract_Event`)))

(event `OnInteract_Event`
  (bind _sequenceplayer (`LevelSequenceActor.SequencePlayer` (`self.Sequence`)))
  (if (and (`self.bInteractable`) (`PrimitiveComponent.IsOverlappingActor` (`self.Sphere`) (`GameplayStatics.GetPlayerPawn` 0)))
    (set `self.bInteracted` true)
    (`SceneComponent.SetVisibility` (`self.Interact`) false false)
    (`self.DisableInput` (`GameplayStatics.GetPlayerPawn` 0) (`GameplayStatics.GetPlayerController` 0))
    (`MovieSceneSequencePlayer.Play` _sequenceplayer)
    (add `MovieSceneSequencePlayer.OnFinished` _sequenceplayer (delegate `OnFinished_Event`))))

(event `OnFinished_Event`
  (`self.EnableInput` (`GameplayStatics.GetPlayerPawn` 0) (`GameplayStatics.GetPlayerController` 0))
  (`self.OnInteracted`))

(event `ShowAndSetInteractable`
  (params (Interactable :type Boolean :default true))
  (bind _output_get (set `self.bInteractable` Interactable))
  (`SceneComponent.SetVisibility` (`self.Interact`) _output_get false))

(event `self.StaticMesh.OnComponentBeginOverlap`
  (params (OverlappedComponent :type "PrimitiveComponent Object Reference") (OtherActor :type "Actor Object Reference") (OtherComp :type "PrimitiveComponent Object Reference") (OtherBodyIndex :type Integer) (bFromSweep :type Boolean) (SweepResult :type "HitResult Structure (by ref)"))
  (if (not (`SceneComponent.bHiddenInGame` (`self.VFX_Statue`)))
    (switch `/Game/MainCharacters/E_MainCharacters` (`self.AOE_Filter`)
      (:`NewEnumerator0`
        (cast `/Game/MainCharacters/BP_AOE_Benelu` OtherActor))
      (:`NewEnumerator1`
        (cast `/Game/MainCharacters/BP_AOE_Kyana` OtherActor))
      (:`NewEnumerator2`
        (cast `/Game/MainCharacters/BP_AOE_Tolg` OtherActor)))
    (set `self.bAttacked` true)
    (`self.OnAttacked`)
    (`ActorComponent.Activate` (`self.VFX_StatueHit`) true)
    (`GameplayStatics.PlaySound2D` "/Game/Placeholder/Audio/curemagic/Cure8.Cure8" 1.0 1.0 0.0 null null)
    (`KismetSystemLibrary.Delay` 0.5)
    (set `self.bAttacked` false)))

(event `self.Sphere.OnComponentBeginOverlap`
  (params (OverlappedComponent :type "PrimitiveComponent Object Reference") (OtherActor :type "Actor Object Reference") (OtherComp :type "PrimitiveComponent Object Reference") (OtherBodyIndex :type Integer) (bFromSweep :type Boolean) (SweepResult :type "HitResult Structure (by ref)"))
  (if (and (`self.bInteractable`) (`self.ActorHasTag` OtherActor "Player"))
    (`SceneComponent.SetVisibility` (`self.Interact`) true false)))

(event `self.Sphere.OnComponentEndOverlap`
  (params (OverlappedComponent :type "PrimitiveComponent Object Reference") (OtherActor :type "Actor Object Reference") (OtherComp :type "PrimitiveComponent Object Reference") (OtherBodyIndex :type Integer))
  (if (and (`self.bInteractable`) (`self.ActorHasTag` OtherActor "Player"))
    (`SceneComponent.SetVisibility` (`self.Interact`) false false)))

(fn `UserConstructionScript`
  (bind _sequence (`self.Sequence`))
  (`parent.UserConstructionScript`)
  (`/Engine/EditorBlueprintResources/StandardMacros.IsValid` _sequence
    (:`Is Valid`
      (`self.K2_SetActorLocation` _sequence (`self.K2_GetActorLocation`) false false))))