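; Destructible dungeon prop that shatters when hit by the player's AOE, swapping its intact static mesh for a Chaos Geometry Collection.
; The construction script applies the mesh and rest collection from variables, so one Blueprint serves different props.
; On hit it moves visibility, collision and physics to the destructed mesh, plays a 2D sound, and spawns and triggers an FS_MasterField at the prop's transform.
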(event `self.OnPlayerAOE_Hit`
  (params (Wheel :type "/Game/Wheel/BP_Wheel Object Reference"))
  (bind _destructedmesh (`self.DestructedMesh`))
  (bind _propsmesh (`self.PropsMesh`))
  (`parent.OnPlayerAOE_Hit` Wheel)
  (`SceneComponent.SetVisibility` _destructedmesh true false)
  (`SceneComponent.SetVisibility` _propsmesh false false)
  (`SceneComponent.SetHiddenInGame` _destructedmesh false false)
  (`PrimitiveComponent.SetSimulatePhysics` _propsmesh false)
  (`PrimitiveComponent.SetCollisionEnabled` _propsmesh "NoCollision")
  (`PrimitiveComponent.SetCollisionEnabled` _destructedmesh "QueryAndPhysics")
  (`PrimitiveComponent.SetSimulatePhysics` _destructedmesh true)
  (`GameplayStatics.PlaySound2D` (`self.Sound`) 0.5 1.0 0.0 null null)
  (bind _returnvalue (`|SpawnActorFromClass` "/Engine/EditorResources/FieldNodes/FS_MasterField.FS_MasterField_C" (`self.GetTransform`) "Undefined" "MultiplyWithRoot" null null))
  (set `/Engine/EditorResources/FieldNodes/FS_MasterField.ActivationType` "NewEnumerator4" _returnvalue)
  (`/Engine/EditorResources/FieldNodes/FS_MasterField.CE_Trigger` _returnvalue))

(fn `UserConstructionScript`
  (`StaticMeshComponent.SetStaticMesh` (`self.PropsMesh`) (`self.New Mesh`))
  (`GeometryCollectionComponent.SetRestCollection` (`self.DestructedMesh`) (`self.Rest Collection In`)))