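; Dungeon trap manager that runs a roulette over a set of symbols, activating a randomly chosen one and repeating after an interval.
; RollSymbol highlights symbols in turn with click sounds through a delayed for-each loop, its delay intended to follow a curve over normalized spin progress.
; A final pass stops on the chosen symbol.
; Activate and Deactivate control the cycle through a Break flag; InitTrap is a to-do stub.
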(event `self.ReceiveBeginPlay`
  (if (`self.ActivateOnSpawn`)
    (`self.RollSymbol`)))

(event `RollSymbol`
  (bind _symbols (`self.Symbols`))
  (set `self.IsRolling` true)
  (set `self.CurTime` 0.0)
  (bind (_array_element _array_index) (`self.ForEachLoopDelay` (`self.Symbols`) (`self.GetCurrentTime`) :!label _label)
    (:`LoopBody`
      (`self.SymbolHandleTurn` _array_element _array_index))
    (:`Completed`
      (if (not (`self.Break`))
        (bind _output_get (set `self.CurTime` (+ (stale _output_get) (/ 1.0 (`self.NbTurns`)))))
        (if (<= _output_get 1.0)
          (goto _label)
          (else
            (bind _output_get_2 (set `self.ChosenSymbol` (`KismetArrayLibrary.Array_Random` _symbols)))
            (bind (_array_element_2 _array_index_2) (`self.ForEachLoopDelay` _symbols (`self.GetCurrentTime`) :!label _label_2)
              (:`LoopBody`
                (`self.SymbolHandleTurn` _array_element_2 _array_index_2)
                (if (== _array_element_2 _output_get_2)
                  (goto _label_2 :!via `Break`)))
              (:`Completed`
                (`/Game/Dungeon/Traps/BP_Symbol.Activate` _output_get_2)
                (`GameplayStatics.PlaySound2D` "/Game/Placeholder/Audio/UI_pack_1/MENU_B_Back.MENU_B_Back" 2.0 1.0 0.0 null null)
                (set `self.IsRolling` false)
                (`KismetSystemLibrary.Delay` (`self.ChoseSymbolInterval`))
                (if (not (`self.Break`))
                  (`self.RollSymbol`))))))
        (else
          (for _array_element_3 (`self.Symbols`)
            (`/Game/Dungeon/Traps/BP_Symbol.SetChosen` _array_element_3 false)))))))

(event `/Game/Dungeon/Traps/BPI_RoomTrap.Deactivate`
  (set `self.Break` true)
  (goto _label :!via `Break`))

(event `/Game/Dungeon/Traps/BPI_RoomTrap.Activate`
  (set `self.Break` false)
  (if (not (`self.IsRolling`))
    (`self.RollSymbol`)))

(event `/Game/Dungeon/Traps/BPI_RoomTrap.InitTrap`
  (params (SigilRoom :type "/Game/Dungeon/BP_SigilRoom Object Reference"))
  (`KismetSystemLibrary.PrintString` "To do : Clamp AOE in AREA"))

(fn `UserConstructionScript`)