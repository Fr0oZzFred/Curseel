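; Trap manager that covers a sigil room with a square grid of fire cells (BP_FireCase) that ignite at random.
; InitTrap destroys old cells, moves to the room and spawns new ones scaled to its size, tagged "Grid".
; A looping timer gives each cell a coin-flip chance to activate, finding cells by a world-wide class and tag search cached when first needed.
; Activate and Deactivate resume or pause that timer.
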(event `/Game/Dungeon/Traps/BPI_RoomTrap.InitTrap`
  (params (SigilRoom :type "/Game/Dungeon/BP_SigilRoom Object Reference"))
  (bind _outactors (`GameplayStatics.GetAllActorsOfClassWithTag` "/Game/Dungeon/Traps/BP_FireCase.BP_FireCase_C" "Grid"))
  (for _array_element _outactors
    (`self.K2_DestroyActor` _array_element))
  (`KismetArrayLibrary.Array_Clear` (`self.FirceCases`))
  (`self.K2_SetActorLocation` (`self.K2_GetActorLocation` SigilRoom))
  (`self.SpawnCases` (`/Game/Dungeon/BP_Room.Size` SigilRoom)))

(event `ToogleSpawn`
  (bind _spawntimer (`self.SpawnTimer`))
  (if (`KismetSystemLibrary.K2_IsTimerPausedHandle` _spawntimer)
    (`KismetSystemLibrary.K2_UnPauseTimerHandle` _spawntimer)
    (else
      (`KismetSystemLibrary.K2_PauseTimerHandle` _spawntimer))))

(event `ActivateSpawn`
  (bind _spawntimer (`self.SpawnTimer`))
  (if (`KismetSystemLibrary.K2_IsTimerPausedHandle` _spawntimer)
    (`KismetSystemLibrary.K2_UnPauseTimerHandle` _spawntimer)))

(event `DeactivateSpawn`
  (bind _spawntimer (`self.SpawnTimer`))
  (if (not (`KismetSystemLibrary.K2_IsTimerPausedHandle` _spawntimer))
    (`KismetSystemLibrary.K2_PauseTimerHandle` _spawntimer)))

(event `self.ReceiveBeginPlay`
  (bind _returnvalue (`KismetSystemLibrary.K2_SetTimerDelegate` (delegate `ActivateCase`) (`self.SpawnIntervalTime`) true))
  (set `self.SpawnTimer` _returnvalue)
  (if (not (`self.ActivateOnSpawn`))
    (`self.ToogleSpawn`)))

(event `ActivateCase`
  (`self.GetFireCases`)
  (for _array_element (`self.FirceCases`)
    (if (`KismetMathLibrary.RandomBool`)
      (`/Game/Dungeon/Traps/BP_FireCase.Activate` _array_element))))

(event `/Game/Dungeon/Traps/BPI_RoomTrap.Activate`
  (`self.ActivateSpawn`))

(event `/Game/Dungeon/Traps/BPI_RoomTrap.Deactivate`
  (`self.DeactivateSpawn`))

(fn `SpawnCases`
  (params (HalfSize :type "Vector Structure"))
  (locals (CaseSize :type "Vector Structure"))
  (bind (_casesize_x _casesize_y) (`KismetMathLibrary.BreakVector` (`local.CaseSize`)))
  (bind _returnvalue (- (`self.CasesNB`) 1))
  (set `local.CaseSize` (/ (* HalfSize 2.0) (`KismetMathLibrary.Conv_IntToDouble` (`self.CasesNB`))))
  (for _index (range (+ _returnvalue 1))
    (for _index_2 (range (+ _returnvalue 1))
      (bind _returnvalue_2 (`|SpawnActorFromClass` "/Game/Dungeon/Traps/BP_FireCase.BP_FireCase_C" (`KismetMathLibrary.MakeTransform` (`KismetMathLibrary.TransformLocation` (`self.GetTransform`) (`KismetMathLibrary.MakeVector` (+ (.x (- (* (`local.CaseSize`) 0.5) (`local.HalfSize`))) (* (`KismetMathLibrary.Conv_IntToDouble` _index_2) _casesize_x)) (+ (.y (- (* (`local.CaseSize`) 0.5) (`local.HalfSize`))) (* (`KismetMathLibrary.Conv_IntToDouble` _index) _casesize_y)) 10.0))) "Undefined" "MultiplyWithRoot" null null))
      (set `Actor.Tags` (`|MakeArray` "Grid" :!type "Name") _returnvalue_2)
      (`/Game/Dungeon/Traps/BP_Symbol.SetSize` _returnvalue_2 (* (`local.CaseSize`) 0.01)))))

(fn `UserConstructionScript`)