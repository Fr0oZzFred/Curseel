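; BP_Case is a resizable dungeon trap element made of a plane, a symbol VFX and a box volume.
; A single Size vector drives the plane's scale, the effect's BoxSize parameter and the box extent, halved in X and Y to fit the plane.
; The construction script applies the sizing, and SetSize stores a new value and reapplies it.
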(fn `SetSize`
  (params (Size :type "Vector Structure"))
  (set `self.Size` Size)
  (`self.UpdateSize`))

(fn `UpdateSize`
  (bind _returnvalue (* (`self.Size`) 100.0))
  (`SceneComponent.SetRelativeScale3D` (`self.Plane`) (`self.Size`))
  (`NiagaraComponent.SetVariableVec3` (`self.VFX_Symbol`) "BoxSize" _returnvalue)
  (`BoxComponent.SetBoxExtent` (`self.Box`) (* _returnvalue (0.5 0.5 1.0)) false))

(fn `UserConstructionScript`
  (`self.UpdateSize`))