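; Fire trap tile that telegraphs, then bursts to damage characters standing on it, either auto-activated on BeginPlay or triggered through Activate.
; A Telegraph timeline drives the fire VFX erosion; on finish it applies GE_SymbolDamage to Box overlaps with a Curseel ASC, shows the symbol, then plays a disappear timeline.
; Sounds use the game mode's SoundManager, polled each tick until valid.
; UpdateSize extends the parent to scale the VFX.
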(event `SetChosen`
  (params (Chosen :type Boolean))
  (bind _sound_manager (`self.Sound Manager`))
  (if Chosen
    (`/Engine/EditorBlueprintResources/StandardMacros.IsValid` _sound_manager
      (:`Is Valid`
        (`/Game/Blueprints/BP_SoundManager.PlayChosenSoundOnce` _sound_manager)))))

(event `self.ReceiveBeginPlay`
  (`|ExecutionSequence`
    (:`then_0`
      (if (`self.AutoActivate`)
        (`self.Activate`)))
    (:`then_1`
      (bind _asgm_in_game (cast `/Game/GameModes/InGame/GM_InGame` (`GameplayStatics.GetGameMode`)))
      (bind _soundmanager (`/Game/GameModes/InGame/GM_InGame.SoundManager` _asgm_in_game))
      (`/Engine/EditorBlueprintResources/StandardMacros.IsValid` _soundmanager :!label _label
        (:`Is Valid`
          (set `self.Sound Manager` _soundmanager))
        (:`Is Not Valid`
          (`KismetSystemLibrary.DelayUntilNextTick`)
          (goto _label))))))

(event `Activate`
  (bind _sound_manager (`self.Sound Manager`))
  (`self.SetChosen` true)
  (bind (_direction _alpha) (`Timeline|Telegraph` :!via `PlayFromStart`)
    (:`Update`
      (`NiagaraComponent.SetVariableFloat` (`self.VFX_FireCase`) "Erosion" _alpha))
    (:`Finished`
      (`|ExecutionSequence`
        (:`then_0`
          (`self.CheckForCharacterCollision`)
          (`NiagaraComponent.SetVariableLinearColor` (`self.VFX_Symbol`) "Color" (make `LinearColor` 1.0 0.0 0.0 1.0))
          (`ActorComponent.Activate` (`self.VFX_Symbol`) true)
          (`self.SetChosen` false)
          (`/Engine/EditorBlueprintResources/StandardMacros.IsValid` _sound_manager
            (:`Is Valid`
              (`/Game/Blueprints/BP_SoundManager.PlayFireSoundOnce` _sound_manager))))
        (:`then_1`
          (bind (_direction_2 _alpha_2) (`Timeline|DisappearAnim` :!via `PlayFromStart`)
            (:`Update`
              (`NiagaraComponent.SetVariableFloat` (`self.VFX_FireCase`) "Erosion" _alpha_2))))))))

(event `CheckForCharacterCollision`
  (for _array_element (`PrimitiveComponent.GetOverlappingActors` (`self.Box`) null)
    (bind _returnvalue (`CurseelBlueprintFunctionLibrary.GetCurseelASC` _array_element))
    (`/Engine/EditorBlueprintResources/StandardMacros.IsValid` _returnvalue
      (:`Is Valid`
        (`CurseelBlueprintFunctionLibrary.ApplyEffect` (make `GameplayEffectApplier` _returnvalue null "Source" "/Game/Dungeon/Traps/GE_SymbolDamage.GE_SymbolDamage_C"))))))

(fn `UpdateSize`
  (bind _size_x (`KismetMathLibrary.BreakVector` (`self.Size`)))
  (`parent.UpdateSize`)
  (`NiagaraComponent.SetVariableFloat` (`self.VFX_FireCase`) "Size" (* _size_x 100.0)))

(fn `UserConstructionScript`
  (`parent.UserConstructionScript`))