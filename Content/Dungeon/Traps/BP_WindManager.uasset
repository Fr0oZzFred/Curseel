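; Dungeon trap manager that spawns BP_AOE_Wind hazards around the player within a sigil room.
; A looping timer spawns each wind at the player's velocity-predicted position plus a random XY offset, clamped to the room range.
; InitTrap moves the manager to the room and derives that range from room size minus a class-default radius.
; Activate resumes the timer, while Deactivate pauses it and destroys all tracked winds.
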(event `RemoveAllPoison`
  (bind _winds (`self.Winds`))
  (for _array_element _winds
    (`/Engine/EditorBlueprintResources/StandardMacros.IsValid` _array_element
      (:`Is Valid`
        (`self.K2_DestroyActor` _array_element))))
  (`KismetArrayLibrary.Array_Clear` _winds))

(event `ToogleSpawn`
  (bind _spawntimer (`self.SpawnTimer`))
  (if (`KismetSystemLibrary.K2_IsTimerPausedHandle` _spawntimer)
    (`KismetSystemLibrary.K2_UnPauseTimerHandle` _spawntimer)
    (else
      (`KismetSystemLibrary.K2_PauseTimerHandle` _spawntimer))))

(event `ActivateSpawn`
  (bind _spawntimer (`self.SpawnTimer`))
  (if (`KismetSystemLibrary.K2_IsTimerPausedHandle` _spawntimer)
    (`KismetSystemLibrary.K2_UnPauseTimerHandle` _spawntimer)))

(event `DeactivateSpawn`
  (bind _spawntimer (`self.SpawnTimer`))
  (if (not (`KismetSystemLibrary.K2_IsTimerPausedHandle` _spawntimer))
    (`KismetSystemLibrary.K2_PauseTimerHandle` _spawntimer)))

(event `self.ReceiveBeginPlay`
  (bind _returnvalue (`KismetSystemLibrary.K2_SetTimerDelegate` (delegate `SpawnWind`) (`self.SpawnIntervalTime`) true))
  (set `self.SpawnTimer` _returnvalue)
  (if (not (`self.ActivateOnSpawn`))
    (`self.ToogleSpawn`)))

(event `SpawnWind`
  (bind _returnvalue (`GameplayStatics.GetPlayerPawn` 0))
  (bind (_returnvalue_x _returnvalue_y) (`KismetMathLibrary.BreakVector` (`self.K2_GetActorLocation`)))
  (bind (_randomoffset_x _randomoffset_y) (`KismetMathLibrary.BreakVector` (`self.RandomOffset`)))
  (bind _rangelimit_x (`KismetMathLibrary.BreakVector2D` (`self.RangeLimit`)))
  (bind (_rangelimit_x_2 _rangelimit_y) (`KismetMathLibrary.BreakVector2D` (`self.RangeLimit`)))
  (bind (_returnvalue_x_2 _returnvalue_y_2) (`KismetMathLibrary.BreakVector` (+ (* (`self.PredictionTime`) (`self.GetVelocity` _returnvalue)) (`self.K2_GetActorLocation` _returnvalue) (`KismetMathLibrary.MakeVector` (`KismetMathLibrary.RandomFloatInRange` (* -1.0 _randomoffset_x) _randomoffset_x) (`KismetMathLibrary.RandomFloatInRange` (* _randomoffset_y -1.0) _randomoffset_y)))))
  (bind _returnvalue_2 (`|SpawnActorFromClass` "/Game/Dungeon/Traps/BP_AOE_Wind.BP_AOE_Wind_C" (`KismetMathLibrary.MakeTransform` (`KismetMathLibrary.MakeVector` (`KismetMathLibrary.FClamp` _returnvalue_x_2 (- _returnvalue_x _rangelimit_x) (+ _rangelimit_x _returnvalue_x)) (`KismetMathLibrary.FClamp` _returnvalue_y_2 (- _returnvalue_y _rangelimit_y) (+ _returnvalue_y _rangelimit_y)))) "AlwaysSpawn" "MultiplyWithRoot" null null))
  (`KismetArrayLibrary.Array_Add` (`self.Winds`) _returnvalue_2))

(event `/Game/Dungeon/Traps/BPI_RoomTrap.Activate`
  (`self.ActivateSpawn`))

(event `/Game/Dungeon/Traps/BPI_RoomTrap.Deactivate`
  (`self.DeactivateSpawn`)
  (`self.RemoveAllPoison`))

(event `/Game/Dungeon/Traps/BPI_RoomTrap.InitTrap`
  (params (SigilRoom :type "/Game/Dungeon/BP_SigilRoom Object Reference"))
  (bind (_size_x _size_y) (`KismetMathLibrary.BreakVector` (`/Game/Dungeon/BP_Room.Size` SigilRoom)))
  (bind _radius (defaults `Object` (`self.Class`)))
  (`self.K2_SetActorLocation` (`self.K2_GetActorLocation` SigilRoom))
  (set `self.RangeLimit` (`KismetMathLibrary.MakeVector2D` (- _size_x _radius) (- _size_y _radius))))

(fn `UserConstructionScript`)