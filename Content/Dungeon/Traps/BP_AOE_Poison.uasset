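; Poison area-of-effect trap, a child of a shared AOE parent, that applies GE_Poison through GAS to filtered actors inside its sphere.
; Radius sizes both visual mesh and collision sphere, and activation can be automatic on BeginPlay.
; A timeline scaled to telegraph duration drives the material's progression, then the snapshot hides the mesh and activates poison VFX.
; Collision checks skip actors already tagged as poisoned and report new hits.
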(event `self.ReceiveBeginPlay`
  (`parent.ReceiveBeginPlay`)
  (`self.UpdateRadius`)
  (if (`self.AutoActivate`)
    (`self.ActivateAOE`)))

(event `self.DisplayTelegraph`
  (`TimelineComponent.SetPlayRate` (`self.TelegraphAnimation`) (/ 1.0 (`self.TelegraphDuration`)))
  (bind (_direction _progression) (`Timeline|TelegraphAnimation` :!via `PlayFromStart`)
    (:`Update`
      (`MeshComponent.SetScalarParameterValueOnMaterials` (`self.VisualMesh`) "Progression" _progression))))

(event `self.ActivateSnapshot`
  (`parent.ActivateSnapshot`)
  (`MeshComponent.SetScalarParameterValueOnMaterials` (`self.VisualMesh`) "Hit" 1.0)
  (`ActorComponent.Activate` (`self.VFX_Poison`) true)
  (`SceneComponent.SetHiddenInGame` (`self.VisualMesh`) true false))

(event `self.CheckForCharactersCollision`
  (`parent.CheckForCharactersCollision`)
  (for _array_element (`PrimitiveComponent.GetOverlappingActors` (`self.Sphere`) (`self.TargetFilter`))
    (`self.ApplyEffect` _array_element)))

(event `ApplyEffect`
  (params (Actor :type "Actor Object Reference"))
  (bind _returnvalue (`CurseelBlueprintFunctionLibrary.GetCurseelASC` Actor))
  (if (not (`GameplayTagAssetInterface.HasMatchingGameplayTag` _returnvalue (struct :`TagName` "State.Debuff.Poison")))
    (`AbilitySystemComponent.BP_ApplyGameplayEffectSpecToSelf` _returnvalue (`AbilitySystemComponent.MakeOutgoingSpec` _returnvalue "/Game/Dungeon/Traps/GE_Poison.GE_Poison_C" 0.0 (`AbilitySystemComponent.MakeEffectContext` _returnvalue)))
    (`self.OnCurseelActorHit` Actor)))

(fn `UpdateRadius`
  (`SceneComponent.SetRelativeScale3D` (`self.VisualMesh`) (`KismetMathLibrary.Conv_DoubleToVector` (* (`self.Radius`) 0.02)))
  (`SphereComponent.SetSphereRadius` (`self.Sphere`) (`self.Radius`) true))

(fn `UserConstructionScript`
  (`parent.UserConstructionScript`)
  (`self.UpdateRadius`))