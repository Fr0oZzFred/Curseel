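; Wind area-of-effect trap, built on a parent AOE, that pulls wheels and monster characters horizontally toward its center.
; A timeline animates the telegraph material, then the snapshot hides it and plays a Niagara wind effect, destroying the actor when finished.
; Collision checks hit each overlapping actor once, replacing its velocity with an inward impulse, stronger for monsters.
; One radius drives the telegraph, collision sphere and effect size.
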(event `self.ReceiveBeginPlay`
  (`parent.ReceiveBeginPlay`)
  (`self.UpdateRadius`)
  (if (`self.AutoActivate`)
    (`self.ActivateAOE`)))

(event `self.DisplayTelegraph`
  (`TimelineComponent.SetPlayRate` (`self.TelegraphAnimation`) (/ 1.0 (`self.TelegraphDuration`)))
  (bind (_direction _progression) (`Timeline|TelegraphAnimation` :!via `PlayFromStart`)
    (:`Update`
      (`MeshComponent.SetScalarParameterValueOnMaterials` (`self.AOE`) "Progression" _progression))))

(event `self.ActivateSnapshot`
  (bind _vfx_wind (`self.VFX_Wind`))
  (bind _aoe (`self.AOE`))
  (`parent.ActivateSnapshot`)
  (`MeshComponent.SetScalarParameterValueOnMaterials` _aoe "Hit" 1.0)
  (`SceneComponent.SetHiddenInGame` _aoe true false)
  (`ActorComponent.Activate` _vfx_wind true)
  (add `NiagaraComponent.OnSystemFinished` _vfx_wind (delegate `OnSystemFinished_Event`)))

(event `OnSystemFinished_Event`
  (params (PSystem :type "NiagaraComponent Object Reference"))
  (`self.K2_DestroyActor`))

(event `self.CheckForCharactersCollision`
  (bind _touchedactor (`self.TouchedActor`))
  (`parent.CheckForCharactersCollision`)
  (for _array_element (`PrimitiveComponent.GetOverlappingActors` (`self.Sphere`) (`self.TargetFilter`))
    (if (== (`KismetArrayLibrary.Array_Find` _touchedactor _array_element) -1)
      (`KismetArrayLibrary.Array_Add` _touchedactor _array_element)
      (`self.ApplyEffect` _array_element))))

(event `ApplyEffect`
  (params (Actor :type "Actor Object Reference"))
  (bind _asbp_wheel (cast `/Game/Wheel/BP_Wheel` Actor)
    (:`then`
      (bind _floatingmovement (`WheelPawn.FloatingMovement` _asbp_wheel))
      (`MovementComponent.StopMovementImmediately` _floatingmovement)
      (set `MovementComponent.Velocity` (* (`KismetMathLibrary.Normal` (- (`self.K2_GetActorLocation`) (`self.K2_GetActorLocation` Actor))) (`KismetMathLibrary.MakeVector` 5000.0 5000.0)) _floatingmovement))
    (:`CastFailed`
      (bind _asbp_monster_character (cast `/Game/Monsters/BP_MonsterCharacter` Actor))
      (bind _charactermovement (`Character.CharacterMovement` _asbp_monster_character))
      (`NavMovementComponent.StopActiveMovement` _charactermovement)
      (set `MovementComponent.Velocity` (* (`KismetMathLibrary.Normal` (- (`self.K2_GetActorLocation`) (`self.K2_GetActorLocation` Actor))) (`KismetMathLibrary.MakeVector` 10000.0 10000.0)) _charactermovement))))

(fn `UpdateRadius`
  (`SceneComponent.SetRelativeScale3D` (`self.AOE`) (`KismetMathLibrary.Conv_DoubleToVector` (* (`self.Radius`) 0.01)))
  (`SphereComponent.SetSphereRadius` (`self.Sphere`) (`self.Radius`) true)
  (`NiagaraComponent.SetVariableFloat` (`self.VFX_Wind`) "Radius" (`self.Radius`)))

(fn `UserConstructionScript`
  (`parent.UserConstructionScript`)
  (`self.UpdateRadius`))